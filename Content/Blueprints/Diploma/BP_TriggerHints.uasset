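; BP_TriggerHints shows a one-time tutorial-style hint on the HUD, started externally through StartHint or ChainHint.
; After an optional delay, it has the BP_HUD_Diploma widget create the message from a table row name and stores the widget's array index.
; A timer later ends the hint by that index and, when chained, triggers the referenced next hint trigger after another delay.
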(event Custom|HintClose
  ;[1 1 1] End
  (Default|EndHint (Variables|/Game/Blueprints/Diploma/BP_HUD_Diploma.BP_HUD_Diploma_C|GetUMG_HUD_ref (stale EventStartHint _asbp_hud_diploma)) (Variables|Default|GetHintArrayIndex))
  (Utilities|Time|ClearandInvalidateTimerbyHandle (stale EventStartHint _returnvalue))
  (if (Variables|Default|GetInChain)
    (Utilities|FlowControl|Delay (Variables|Default|GetDelayForNext))
    (Default|ChainHint (Variables|Default|GetBP_TriggerHint))))

(event EventBeginPlay)

(event Collision|EventActorBeginOverlap
  (params (OtherActor :type Actor%20Object%20Reference)))

(event EventTick
  (params (DeltaSeconds :type Float%20%28single-precision%29)))

(event EventStartHint
  ;[1 1 1] Create hint
  (if (Variables|Default|GetNeedDelay)
    (Utilities|FlowControl|Delay (Variables|Default|GetDelayBeforeHint)))
  (if (not (Variables|Default|GetIsExists))
    (Variables|Default|SetIsExists true)
    (bind _asbp_hud_diploma (Utilities|Casting|CastToBP_HUD_Diploma (HUD|GetHUD (Game|GetPlayerController 0))))
    (Variables|Default|SetHintArrayIndex (Variables|/Game/UI/UMG_HUD.UMG_HUD_C|GetArrayIndex (Variables|/Game/Blueprints/Diploma/BP_HUD_Diploma.BP_HUD_Diploma_C|GetUMG_HUD_ref _asbp_hud_diploma)))
    (Class|BPIHints|CreateHint(Message) (Variables|/Game/Blueprints/Diploma/BP_HUD_Diploma.BP_HUD_Diploma_C|GetUMG_HUD_ref _asbp_hud_diploma) (Variables|Default|GetHint%20Table%20Row%20Name))
    ;[1 1 1] End
    (bind _returnvalue (Utilities|Time|SetTimerbyEvent (delegate Custom|HintClose) (Variables|Default|GetHintDuration)))))

(event EventChainHint
  ;[1 1 1] Create hint
  (if (Variables|Default|GetNeedDelay)
    (Utilities|FlowControl|Delay (Variables|Default|GetDelayBeforeHint)))
  (if (not (Variables|Default|GetIsExists))
    (Variables|Default|SetIsExists true)
    (bind _asbp_hud_diploma (Utilities|Casting|CastToBP_HUD_Diploma (HUD|GetHUD (Game|GetPlayerController 0))))
    (Variables|Default|SetHintArrayIndex (Variables|/Game/UI/UMG_HUD.UMG_HUD_C|GetArrayIndex (Variables|/Game/Blueprints/Diploma/BP_HUD_Diploma.BP_HUD_Diploma_C|GetUMG_HUD_ref _asbp_hud_diploma)))
    (Class|BPIHints|CreateHint(Message) (Variables|/Game/Blueprints/Diploma/BP_HUD_Diploma.BP_HUD_Diploma_C|GetUMG_HUD_ref _asbp_hud_diploma) (Variables|Default|GetHint%20Table%20Row%20Name))
    ;[1 1 1] End
    (bind _returnvalue (Utilities|Time|SetTimerbyEvent (delegate Custom|HintClose) (Variables|Default|GetHintDuration)))))

(fn ConstructionScript)

(fn IsNeed
  (return false))