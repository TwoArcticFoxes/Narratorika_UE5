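; BP_Timer is an interactable timer actor that triggers a linked ControlActor after a countdown.
; On BeginPlay it passes itself to the W_TimerButton in its widget component.
; InteractInterface starts a looping one-second timer, ignoring repeat presses while InProcess is set.
; When CountdownProgress equals CountdownDuration, it calls ControlInterface on ControlActor after a short delay, then waits before clearing the timer and resetting.
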(event Custom|Countdown
  (Math|Float|IncrementFloat (Variables|Default|GetCountdownProgress)
    (:%20%20
      (if (== (Variables|Default|GetCountdownDuration) (Variables|Default|GetCountdownProgress))
        (Utilities|FlowControl|Delay 0.2)
        (Default|ControlInterface (Variables|Default|GetControlActor))
        (Utilities|FlowControl|Delay 5.0)
        (Utilities|Time|ClearandInvalidateTimerbyHandle (Variables|Default|GetTimer))
        (Variables|Default|SetCountdownProgress 0.0)
        (Variables|Default|SetInProcess false)))))

(event EventBeginPlay
  (|CallParentFunction)
  (bind _asw_timer_button (Utilities|Casting|CastToW_TimerButton (UserInterface|GetUserWidgetObject (Variables|Default|GetWidget))))
  (Variables|/Game/UI/BPWidgets/W_TimerButton.W_TimerButton_C|SetTimerButtonRef _asw_timer_button self))

(event Collision|EventActorBeginOverlap
  (params (OtherActor :type Actor%20Object%20Reference))
  (|CallParentFunction OtherActor) ; This node is disabled and will not be called.\nDrag off pins to build functionality.
)

(event EventTick
  (params (DeltaSeconds :type Float%20%28single-precision%29))
  (|CallParentFunction DeltaSeconds) ; This node is disabled and will not be called.\nDrag off pins to build functionality.
)

(event EventInteractInterface
  (if (not (Variables|Default|GetInProcess))
    (Variables|Default|SetInProcess true)
    (bind _returnvalue (Utilities|Time|SetTimerbyEvent (delegate Custom|Countdown) 1.0 true))
    (Variables|Default|SetTimer _returnvalue)))

(fn ConstructionScript
  (|CallParentFunction))