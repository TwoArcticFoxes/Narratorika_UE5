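; BP_CameraCharacter is a possessable camera that the player looks through and scans from.
; NeedPossess has player controller 0 possess it, then PossessCamera clears existing widgets, shows either the normal or broken-camera HUD based on IsNeedFix, and adds the Enhanced Input context.
; Look input turns the view, and scanner input triggers BPScanner's scanner mode with its camera.
; CheckStatus reports whether it is neither turned off nor broken.
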(event Custom|PossessCamera
  (Viewport|RemoveAllWidgets)
  (Utilities|FlowControl|Sequence
    (:then_0
      ;[1 1 1] HUD
      (if (Variables|Default|GetIsNeedFix)
        (bind _returnvalue (UserInterface|CreateWidget "/Game/UI/UMG_HUD_BrokenCamera.UMG_HUD_BrokenCamera_C"))
        (UserInterface|Viewport|AddtoViewport _returnvalue 0)
        (else
          (bind _returnvalue_2 (UserInterface|CreateWidget "/Game/UI/UMG_HUD_CameraCharacter.UMG_HUD_CameraCharacter_C"))
          (UserInterface|Viewport|AddtoViewport _returnvalue_2 0))))
    (:then_1
      ;[1 1 1] Camera
      (bind _asplayer_controller (Utilities|Casting|CastToPlayerController (Pawn|GetController)))
      (Utilities|IsValid (PlayerController|LocalPlayerSubsystems|GetEnhancedInputLocalPlayerSubsystem _asplayer_controller)
        (:Is%20Valid
          (Input|AddMappingContext (PlayerController|LocalPlayerSubsystems|GetEnhancedInputLocalPlayerSubsystem _asplayer_controller) "/Game/ThirdPerson/Input/IMC_Default.IMC_Default" 0 "(bIgnoreAllPressedKeysUntilRelease=True,bForceImmediately=False)"))))))

(event Input|EnhancedActionEvents|EnhancedInputActionIA_Look
  (params (ActionValue :type Vector%202D%20Structure) (ElapsedSeconds :type Float%20%28double-precision%29) (TriggeredSeconds :type Float%20%28double-precision%29) (InputAction :type Input%20Action%20Object%20Reference :default "/Game/ThirdPerson/Input/Actions/IA_Look.IA_Look"))
  ;[1 1 1] Camera
  ;;[1 1 1] Mouse
  (:Triggered
    (Pawn|Input|AddControllerYawInput (.x ActionValue))
    (Pawn|Input|AddControllerPitchInput (.y ActionValue))))

(event Input|EnhancedActionEvents|EnhancedInputActionIA_Scanner
  (params (ActionValue :type Boolean) (ElapsedSeconds :type Float%20%28double-precision%29) (TriggeredSeconds :type Float%20%28double-precision%29) (InputAction :type Input%20Action%20Object%20Reference :default "/Game/ThirdPerson/Input/Actions/IA_Scanner.IA_Scanner"))
  ;[1 1 1] Scanner
  (:Started
    (Default|ScannerMode (Variables|Default|GetBP_Scanner) (Variables|Default|GetCamera))))

(event EventNeedPossess
  ;[1 1 1] Possess
  (Pawn|Possess (Game|GetPlayerController 0) self)
  (CallFunction|PossessCamera))

(fn ConstructionScript)

(fn CheckStatus
  (return (and (not (Variables|Default|GetIsTurnOff)) (not (Variables|Default|GetIsBroken)))))