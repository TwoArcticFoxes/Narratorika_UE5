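; Pause menu Blueprint that toggles the game's pause screen from the IA_InGameMenu input action.
; A FlipFlop alternates between creating UMG_PauseMenu, then pausing with UI-only input and cursor after a short delay, and removing it to restore gameplay.
; The widget's Continue event is bound to EndWidget, which jumps into the same closing path without advancing the FlipFlop.
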(event Custom|EndWidget
  (bind _returnvalue (Game|GetPlayerController 0))
  (Widget|RemovefromParent (stale Input|EnhancedActionEvents|EnhancedInputActionIA_InGameMenu _returnvalue_2))
  (Game|SetGamePaused false)
  (Input|SetInputModeGameOnly _returnvalue false)
  (Variables|/Script/Engine.PlayerController|SetbShowMouseCursor _returnvalue false))

(event Input|EnhancedActionEvents|EnhancedInputActionIA_InGameMenu
  (params (ActionValue :type Boolean) (ElapsedSeconds :type Float%20%28double-precision%29) (TriggeredSeconds :type Float%20%28double-precision%29) (InputAction :type Input%20Action%20Object%20Reference :default "/Game/ThirdPerson/Input/Actions/IA_InGameMenu.IA_InGameMenu"))
  (bind _returnvalue (Game|GetPlayerController 0))
  (:Started
    (Utilities|FlowControl|FlipFlop
      (:A
        (bind _returnvalue_2 (UserInterface|CreateWidget "/Game/UI/Homework/UMG_PauseMenu.UMG_PauseMenu_C"))
        (EventDispatchers|BindEventtoPauseMenuContinue _returnvalue_2 (delegate Custom|EndWidget))
        (UserInterface|Viewport|AddtoViewport _returnvalue_2 0)
        (Utilities|FlowControl|Delay 0.2)
        (Game|SetGamePaused true)
        (Input|SetInputModeUIOnly _returnvalue 0 "DoNotLock" false)
        (Variables|/Script/Engine.PlayerController|SetbShowMouseCursor _returnvalue true))
      (:B
        (Development|PrintString (Utilities|GetDisplayName _returnvalue_2))
        (Widget|RemovefromParent _returnvalue_2)
        (Game|SetGamePaused false)
        (Input|SetInputModeGameOnly _returnvalue false)
        (Variables|/Script/Engine.PlayerController|SetbShowMouseCursor _returnvalue false)))))