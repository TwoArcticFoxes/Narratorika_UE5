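; BP_Scanner is a toggleable scanner mode that finds interactive and possessable objects in front of a supplied camera.
; Toggling on shows the UMG_scanner widget and starts a looping line-trace timer; toggling off removes both.
; Hits implementing BPI_InteractiveObject receive a light message, while BPI_possess hits open a gate.
; IA_Interact passes through that gate to stop tracing and send the hit actor a possess message.
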(event Custom|SelectItem
  ;[1 1 1] Select Item Event
  (bind _returnvalue (Utilities|Time|SetTimerbyEvent (delegate Custom|Line%20trace) 0.3 true))
  (Variables|Default|SetTimerScanner _returnvalue))

(event Custom|Line%20trace
  (bind _camera (Variables|Default|GetCamera))
  (bind _returnvalue (Transformation|GetWorldLocation _camera))
  (bind _returnvalue_2 (Math|Vector|GetForwardVector _camera))
  ;[1 1 1] Select Item Event
  ;;[1 1 1] LineTraceTimer
  (bind (_outhit _returnvalue_3) (Collision|LineTraceByChannel (+ _returnvalue (* (Variables|Default|GetStartDistance) _returnvalue_2)) (+ _returnvalue (* _returnvalue_2 (Variables|Default|GetDistanceTrace))) "TraceTypeQuery1" false 0 "None"))
  (Variables|Default|SetHit%20Actor (.HitActor (Collision|BreakHitResult _outhit)))
  (if _returnvalue_3
    (Development|PrintString (Utilities|GetDisplayName (Variables|Default|GetHit%20Actor)))
    (Utilities|FlowControl|Sequence
      (:then_0
        ;;[1 1 1] Light
        (if (Utilities|DoesObjectImplementInterface (Variables|Default|GetHit%20Actor) "/Game/Blueprints/BPI/BPI_InteractiveObject.BPI_InteractiveObject_C")
          (Class|BPIInteractiveObject|LightInterface(Message) (Variables|Default|GetHit%20Actor))))
      (:then_1
        ;;[1 1 1] Possess
        (if (Utilities|DoesObjectImplementInterface (Variables|Default|GetHit%20Actor) "/Game/Blueprints/BPI/BPI_possess.BPI_possess_C")
          (Utilities|FlowControl|Gate true) ; enters at Open
          (else
            (Utilities|FlowControl|Gate true) ; enters at Close
          ))))))

(event Custom|ScannerMode
  (params (Camera :type Camera%20Component%20Object%20Reference))
  ;[1 1 1] Activate
  (Variables|Default|SetCamera Camera)
  (Utilities|FlowControl|FlipFlop
    (:A
      (Variables|Default|SetIsScannerOpen true)
      (bind _returnvalue (UserInterface|CreateWidget "/Game/UI/UMG_scanner.UMG_scanner_C"))
      (bind _output_get (Variables|Default|SetUMG_Scanner _returnvalue))
      (UserInterface|Viewport|AddtoViewport _returnvalue 0)
      (CallFunction|SelectItem))
    (:B
      (Variables|Default|SetIsScannerOpen false)
      (Widget|RemovefromParent (Variables|Default|GetUMG_Scanner))
      (Utilities|Time|ClearandInvalidateTimerbyHandle (Variables|Default|GetTimerScanner)))))

(event Input|EnhancedActionEvents|EnhancedInputActionIA_Interact
  (params (ActionValue :type Boolean) (ElapsedSeconds :type Float%20%28double-precision%29) (TriggeredSeconds :type Float%20%28double-precision%29) (InputAction :type Input%20Action%20Object%20Reference :default "/Game/ThirdPerson/Input/Actions/IA_Interact.IA_Interact"))
  ;[1 1 1] Select Item Event
  ;;[1 1 1] Possess
  (:Started
    (Utilities|FlowControl|Gate true
      (:Exit
        (Utilities|FlowControl|Sequence
          (:then_0
            (Utilities|Time|ClearandInvalidateTimerbyHandle (Variables|Default|GetTimerScanner)))
          (:then_1
            (Class|BPIPossess|NeedPossess(Message) (Variables|Default|GetHit%20Actor)))
          (:then_2
            (Variables|Default|SetHit%20Actor 0))
          (:then_3
            (Variables|Default|SetIsScannerOpen false)))))))