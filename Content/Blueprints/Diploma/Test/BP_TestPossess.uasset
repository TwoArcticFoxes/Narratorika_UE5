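; BP_TestPossess is a test Blueprint with a cube that responds to interact and light interface events.
; Interacting calls PossessCamera, apparently an event dispatcher whose listeners are not defined here.
; The light event swaps the cube's material to a gold prototype grid.
; BeginPlay, overlap, Tick and construction add no logic of their own.
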(event EventBeginPlay
  (|CallParentFunction) ; This node is disabled and will not be called.\nDrag off pins to build functionality.
)

(event Collision|EventActorBeginOverlap
  (params (OtherActor :type Actor%20Object%20Reference))
  (|CallParentFunction OtherActor) ; This node is disabled and will not be called.\nDrag off pins to build functionality.
)

(event EventTick
  (params (DeltaSeconds :type Float%20%28single-precision%29))
  (|CallParentFunction DeltaSeconds) ; This node is disabled and will not be called.\nDrag off pins to build functionality.
)

(event EventLightInterface
  (Rendering|Material|SetMaterial (Variables|Default|GetCube) 0 "/Game/LevelPrototyping/Materials/MI_PrototypeGrid_Gold.MI_PrototypeGrid_Gold"))

(event EventInteractInterface
  (Default|CallPossessCamera))

(fn ConstructionScript
  (|CallParentFunction))