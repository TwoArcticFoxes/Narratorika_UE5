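; Interactable test computer that opens a start-computer dialogue and records how the conversation ends.
; On interaction it clears the widgets, shows the dialogue fed by its data table and switches to UI-only input with a cursor.
; When the dialogue ends, it restores the HUD and game input, then maps the answer ID to welcome, angry and complete flags on BP_GameModLessons.
; The non-angry endings also call the camera possession event.
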(event Custom|DialogueEnd
  (params (IDAnswer :type Integer))
  (bind _returnvalue (Game|GetPlayerController 0))
  ;[1 1 1] DialogueWidget
  ;;[1 1 1] Remove Widget
  (Utilities|FlowControl|Sequence
    (:then_0
      (Widget|RemovefromParent (stale EventInteractInterface _returnvalue_2))
      (bind _returnvalue_2 (UserInterface|CreateWidget "/Game/UI/Homework/UMG_HUD_testground.UMG_HUD_testground_C"))
      (UserInterface|Viewport|AddtoViewport _returnvalue_2 0)
      (Input|SetInputModeGameOnly _returnvalue false)
      (Variables|/Script/Engine.PlayerController|SetbShowMouseCursor _returnvalue false))
    (:then_1
      ;;[1 1 1] Варианты завершения
      (bind _asbp_game_mod_lessons (Utilities|Casting|CastToBP_GameModLessons (Game|GetGameMode)))
      (switch int IDAnswer
        (:-3
          (Variables|/Game/Blueprints/BP_GameModLessons.BP_GameModLessons_C|SetIs%20Welcome _asbp_game_mod_lessons false)
          (Variables|/Game/Blueprints/BP_GameModLessons.BP_GameModLessons_C|SetIs%20Angry _asbp_game_mod_lessons false)
          (Variables|/Game/Blueprints/BP_GameModLessons.BP_GameModLessons_C|SetIs%20Complete _asbp_game_mod_lessons true)
          (Default|CallPossesstoCamera :!label _label))
        (:-2
          (Variables|/Game/Blueprints/BP_GameModLessons.BP_GameModLessons_C|SetIs%20Welcome _asbp_game_mod_lessons true)
          (Variables|/Game/Blueprints/BP_GameModLessons.BP_GameModLessons_C|SetIs%20Angry _asbp_game_mod_lessons true)
          (Variables|/Game/Blueprints/BP_GameModLessons.BP_GameModLessons_C|SetIs%20Complete _asbp_game_mod_lessons false))
        (:-1
          (Variables|/Game/Blueprints/BP_GameModLessons.BP_GameModLessons_C|SetIs%20Welcome _asbp_game_mod_lessons true)
          (Variables|/Game/Blueprints/BP_GameModLessons.BP_GameModLessons_C|SetIs%20Angry _asbp_game_mod_lessons false)
          (Variables|/Game/Blueprints/BP_GameModLessons.BP_GameModLessons_C|SetIs%20Complete _asbp_game_mod_lessons false)
          (goto _label))))))

(event EventInteractInterface
  (bind _returnvalue (Game|GetPlayerController 0))
  ;[1 1 1] DialogueWidget
  ;;[1 1 1] CreateWidget
  (Viewport|RemoveAllWidgets)
  (bind _returnvalue_2 (UserInterface|CreateWidget "/Game/UI/Homework/UMG_StartComputerDialoge.UMG_StartComputerDialoge_C" _returnvalue (Variables|Default|GetDialogueDataTable)))
  (EventDispatchers|BindEventtoEndDialogue _returnvalue_2 (delegate Custom|DialogueEnd))
  (UserInterface|Viewport|AddtoViewport _returnvalue_2 0)
  (Input|SetInputModeUIOnly _returnvalue 0 "DoNotLock" true)
  (Variables|/Script/Engine.PlayerController|SetbShowMouseCursor _returnvalue true))

(fn ConstructionScript
  (|CallParentFunction))