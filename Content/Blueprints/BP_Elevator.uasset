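; Elevator actor that moves from its placed position to a relative offset when triggered through a control interface event.
; BeginPlay turns the offset into a world end point, and the trigger starts a timeline after a delay, lerping location without sweep at an adjustable play rate.
; An IsMoved flag blocks retriggering; with IsRepeat the endpoints swap on finish and the flag clears, so the next trigger sends it back.
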(event Custom|StartMoving
  ;[1 1 1] StartMoving Timeline
  (CallFunction|PlayRateFunction)
  (bind _moving (Timeline|MovingTimeline PlayFromStart)
    (:Update
      (Transformation|SetActorLocation (Math|Vector|Lerp(Vector) (Variables|Default|GetStartLocation) (Variables|Default|GetEndLocation) _moving) false false))
    (:Finished
      (if (Variables|MovingTimeline|GetIsRepeat)
        (Variables|Default|SetTempLocation (Variables|Default|GetStartLocation))
        (Variables|Default|SetStartLocation (Variables|Default|GetEndLocation))
        (Variables|Default|SetEndLocation (Variables|Default|GetTempLocation))
        (Variables|Control|SetIsMoved false)))))

(event EventBeginPlay
  ;[1 1 1] BeginPlay
  (|CallParentFunction)
  (bind _output_get (Variables|Default|SetStartLocation (Transformation|GetActorLocation)))
  (Variables|Default|SetEndLocation (+ _output_get (Variables|Default|GetEndLocation))))

(event EventControlInterface
  ;[1 1 1] Control
  (if (not (Variables|Control|GetIsMoved))
    (Variables|Control|SetIsMoved true)
    (Utilities|FlowControl|Delay (Variables|Control|GetDelay))
    (CallFunction|StartMoving)))

(fn ConstructionScript
  (|CallParentFunction))

(fn PlayRateFunction
  (Components|Timeline|SetPlayRate (Variables|Default|GetMovingTimeline) (/ (Variables|MovingTimeline|GetPlayRate) (Variables|MovingTimeline|GetPlayRateMod))))