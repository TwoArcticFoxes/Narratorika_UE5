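; BP_Cube is a moving cube that sweeps back and forth between its spawn point and an offset, damaging the player character on hit.
; A timeline with adjustable play rate lerps its location, swapping endpoints on each finish.
; Hits from other actors, including cubes, recolor it, then after a delay DestroyCube increments the GameMode's cube counter and destroys it.
; Character hits lower GameMode health; overlaps only print debug text.
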(event OnComponentHit(Cube)
  (params (HitComponent :type Primitive%20Component%20Object%20Reference) (OtherActor :type Actor%20Object%20Reference) (OtherComp :type Primitive%20Component%20Object%20Reference) (NormalImpulse :type Vector :default "0, 0, 0") (Hit :type Hit%20Result%20Structure%20%28by%20ref%29))
  ;[1 1 1] Hit
  ;;[1 1 1] Destroy by self
  (Utilities|Casting|CastToBP_Cube OtherActor
    (:then
      (Rendering|Material|SetMaterial (Variables|Default|GetCube) 0 "/Game/LevelPrototyping/Materials/MI_PrototypeGrid_Yellow.MI_PrototypeGrid_Yellow")
      (Utilities|FlowControl|Delay 0.3)
      (CallFunction|DestroyCube))
    (:CastFailed
      ;;[1 1 1] BP_Person
      (Utilities|Casting|CastToBP_ThirdPersonCharacter OtherActor
        (:then
          (bind _asbp_game_mode (Utilities|Casting|CastToBP_GameMode (Game|GetGameMode)))
          (bind _output_get (Variables|/Game/Blueprints/BP_GameMode.BP_GameMode_C|SetCharacterHealth _asbp_game_mode (- (Variables|/Game/Blueprints/BP_GameMode.BP_GameMode_C|GetCharacterHealth _asbp_game_mode) 0.1)))
          (Development|PrintString (Utilities|String|ToString(Float) _output_get)))
        (:CastFailed
          ;;[1 1 1] Destroy by other
          (Rendering|Material|SetMaterial (Variables|Default|GetCube) 0 "/Game/LevelPrototyping/Materials/MI_PrototypeGrid_Red.MI_PrototypeGrid_Red")
          (Utilities|FlowControl|Delay 0.3)
          (CallFunction|DestroyCube))))))

(event OnComponentBeginOverlap(Cube)
  (params (OverlappedComponent :type Primitive%20Component%20Object%20Reference) (OtherActor :type Actor%20Object%20Reference) (OtherComp :type Primitive%20Component%20Object%20Reference) (OtherBodyIndex :type Integer) (bFromSweep :type Boolean) (SweepResult :type Hit%20Result%20Structure%20%28by%20ref%29))
  ;[0.05937 0.05937 0.05937] Overlap test
  (Utilities|Casting|CastToBP_Cube OtherActor
    (:then
      (Development|PrintString "Overlap BP_Cube" true true "(R=0.000000,G=0.660000,B=1.000000,A=1.000000)" 1e+01))
    (:CastFailed
      (Utilities|Casting|CastToBP_ThirdPersonCharacter OtherActor
        (:then
          (Development|PrintString "Overlap PersonChatracter" true true "(R=0.000000,G=1.000000,B=0.034738,A=1.000000)"))
        (:CastFailed
          (Utilities|Casting|CastToBP_sphere OtherActor
            (:then
              (Development|PrintString "Overlap BP_sphere" true true "(R=1.000000,G=0.927710,B=0.000000,A=1.000000)"))
            (:CastFailed
              (Development|PrintString "Overlap Other" true true "(R=1.000000,G=0.000000,B=0.001717,A=1.000000)"))))))))

(event Custom|StartMoving
  ;[1 1 1] Moving
  ;;[1 1 1] StartMoving Timeline
  (Components|Timeline|SetPlayRate (Variables|Default|GetMoving%20Timeline) (/ (Variables|Default|GetPlayRateTimeline) (Variables|Default|GetPlayRateTimelineMod)))
  (bind _moving (Timeline|Moving%20Timeline PlayFromStart)
    (:Update
      (Transformation|SetActorLocation (Math|Vector|Lerp(Vector) (Variables|Default|GetStartLocation) (Variables|Default|GetEndLocation) _moving) true false))
    (:Finished
      (Variables|Default|SetTempLocation (Variables|Default|GetStartLocation))
      (Variables|Default|SetStartLocation (Variables|Default|GetEndLocation))
      (Variables|Default|SetEndLocation (Variables|Default|GetTempLocation))
      (CallFunction|StartMoving))))

(event EventBeginPlay
  ;[1 1 1] Moving
  ;;[1 1 1] Begin play
  (bind _output_get (Variables|Default|SetStartLocation (Transformation|GetActorLocation)))
  (Variables|Default|SetEndLocation (+ _output_get (Variables|Default|GetEndLocation)))
  (CallFunction|StartMoving))

(fn ConstructionScript)

(fn DestroyCube
  (bind _asbp_game_mode (Utilities|Casting|CastToBP_GameMode (Game|GetGameMode)))
  (Math|Integer|IncrementInt (Variables|/Game/Blueprints/BP_GameMode.BP_GameMode_C|GetNumberOfCubes _asbp_game_mode)
    (:%20%20
      (Actor|DestroyActor))))