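; BP_TriggerText is an interactive trigger actor that displays configurable text through a TextRender component.
; Its Control event waits for a delay, sets the text, then calls Control on ControlActor when chaining is enabled.
; When the interactive actor overlap ends, temporary text is cleared.
; Tick reapplies the configured world size to the text every frame.
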(event EventBeginPlay
  (|CallParentFunction) ; This node is disabled and will not be called.\nDrag off pins to build functionality.
)

(event Collision|EventActorBeginOverlap
  (params (OtherActor :type Actor%20Object%20Reference))
  (|CallParentFunction OtherActor) ; This node is disabled and will not be called.\nDrag off pins to build functionality.
)

(event EventTick
  (params (DeltaSeconds :type Float%20%28single-precision%29))
  (|CallParentFunction DeltaSeconds)
  (Rendering|Components|TextRender|SetWorldSize (Variables|Default|GetTextRender) (Variables|Default|GetTextSize)))

(event EventControl
  (Utilities|FlowControl|Delay (Variables|Default|GetDelay))
  (bind _output_get (Variables|Default|SetTempText (Variables|Default|GetText)))
  (Rendering|Components|TextRender|SetText (Variables|Default|GetTextRender) _output_get)
  (if (Variables|Default|GetIsChain)
    (Default|Control (Variables|Default|GetControlActor))))

(event EventEndOverlapInteractiveActor
  (if (Variables|Default|GetIsTemp)
    (bind _output_get (Variables|Default|SetTempText ""))
    (Rendering|Components|TextRender|SetText (Variables|Default|GetTextRender) _output_get)))

(fn ConstructionScript
  (|CallParentFunction))