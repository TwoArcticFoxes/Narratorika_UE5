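; BP_Key is a collectible key actor that spins until the player interacts with it.
; Tick drives both roll and yaw from the current roll, advanced by base speed times a speed modifier and delta time.
; Interact increments the key count in BP_GameMode, destroys the key, and calls Control on a linked ControlActor when IsChain is set.
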(event EventBeginPlay
  (|CallParentFunction) ; This node is disabled and will not be called.\nDrag off pins to build functionality.
)

(event Collision|EventActorBeginOverlap
  (params (OtherActor :type Actor%20Object%20Reference))
  (|CallParentFunction OtherActor) ; This node is disabled and will not be called.\nDrag off pins to build functionality.
)

(event EventTick
  (params (DeltaSeconds :type Float%20%28single-precision%29))
  (bind _returnvalue (Transformation|GetActorRotation))
  (bind _basespeedrotation (Variables|Default|GetBaseSpeedRotation))
  (bind _speedmod (Variables|Default|GetSpeedMod))
  (bind _returnvalue_2 (* _basespeedrotation _speedmod))
  (bind _returnvalue_3 (* DeltaSeconds _returnvalue_2))
  (bind _returnvalue_4 (+ _returnvalue_3 (.roll _returnvalue)))
  ;[1 1 1] Rotation
  (Transformation|SetActorRotation (Math|Rotator|MakeRotator _returnvalue_4 0.0 _returnvalue_4)))

(event EventInteract
  ;[1 1 1] Interact
  (bind _asbp_game_mode (Utilities|Casting|CastToBP_GameMode (Game|GetGameMode)))
  (Math|Integer|IncrementInt (Variables|/Game/Blueprints/Lesson_4/BP_GameMode.BP_GameMode_C|GetKeys _asbp_game_mode)
    (:%20%20
      (Actor|DestroyActor)
      (if (Variables|Default|GetIsChain)
        (Default|Control (Variables|Default|GetControlActor))))))

(fn ConstructionScript
  (|CallParentFunction))