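; Interactive door actor that toggles between open and closed when its Interact event fires.
; An IsOpen flag picks the branch, which snaps the whole actor to either zero rotation or a 90-degree turn and flips the flag.
; Rotations are absolute world values with no interpolation, so the door ignores its placed orientation.
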(event EventBeginPlay
  (|CallParentFunction) ; This node is disabled and will not be called.\nDrag off pins to build functionality.
)

(event Collision|EventActorBeginOverlap
  (params (OtherActor :type Actor%20Object%20Reference))
  (|CallParentFunction OtherActor) ; This node is disabled and will not be called.\nDrag off pins to build functionality.
)

(event EventTick
  (params (DeltaSeconds :type Float%20%28single-precision%29))
  (|CallParentFunction DeltaSeconds) ; This node is disabled and will not be called.\nDrag off pins to build functionality.
)

(event EventInteract
  (if (Variables|Default|GetIsOpen)
    (Transformation|SetActorRotation "0.000000,0.000000,0.000000")
    (Variables|Default|SetIsOpen false)
    (else
      (Transformation|SetActorRotation "0.000000,90.000000,0.000000")
      (Variables|Default|SetIsOpen true))))

(fn ConstructionScript
  (|CallParentFunction))