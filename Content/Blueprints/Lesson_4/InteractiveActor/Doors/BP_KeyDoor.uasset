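; BP_KeyDoor is an interactive door that takes a key to open.
; On Interact it casts the game mode to BP_GameMode and, if the Keys count stored there is above zero, spends one and snaps the actor to a fixed absolute rotation.
; It keeps no opened state, so each further interaction consumes another key while any remain.
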(event EventBeginPlay
  (|CallParentFunction) ; This node is disabled and will not be called.\nDrag off pins to build functionality.
)

(event Collision|EventActorBeginOverlap
  (params (OtherActor :type Actor%20Object%20Reference))
  (|CallParentFunction OtherActor) ; This node is disabled and will not be called.\nDrag off pins to build functionality.
)

(event EventTick
  (params (DeltaSeconds :type Float%20%28single-precision%29))
  (|CallParentFunction DeltaSeconds) ; This node is disabled and will not be called.\nDrag off pins to build functionality.
)

(event EventInteract
  (bind _asbp_game_mode (Utilities|Casting|CastToBP_GameMode (Game|GetGameMode)))
  (if (> (Variables|/Game/Blueprints/BP_GameMode.BP_GameMode_C|GetKeys _asbp_game_mode) 0)
    (Math|Integer|DecrementInt (Variables|/Game/Blueprints/BP_GameMode.BP_GameMode_C|GetKeys _asbp_game_mode)
      (:%20%20
        (Transformation|SetActorRotation "0.000000,90.000000,0.000000")))))

(fn ConstructionScript
  (|CallParentFunction))