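; BP_LightPoint is an interactive spot light that can be switched on and off and can take part in a chain of controlled actors.
; At BeginPlay, after the parent logic, the spot light's visibility is set from IsLight.
; The Control event waits for a configurable delay, toggles the light, then forwards Control to ControlActor when IsChain is set, producing staggered sequences.
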(event EventBeginPlay
  ;[1 1 1] BeginPlay
  (|CallParentFunction)
  (Rendering|SetVisibility (Variables|Default|GetSpotLight) (Variables|Default|GetIsLight) false))

(event Collision|EventActorBeginOverlap
  (params (OtherActor :type Actor%20Object%20Reference))
  (|CallParentFunction OtherActor) ; This node is disabled and will not be called.\nDrag off pins to build functionality.
)

(event EventTick
  (params (DeltaSeconds :type Float%20%28single-precision%29))
  (|CallParentFunction DeltaSeconds) ; This node is disabled and will not be called.\nDrag off pins to build functionality.
)

(event EventControl
  ;[1 1 1] Control
  (Utilities|FlowControl|Delay (Variables|Default|GetDelay))
  (Rendering|ToggleVisibility (Variables|Default|GetSpotLight) false)
  (if (Variables|Default|GetIsChain)
    (Default|Control (Variables|Default|GetControlActor))))

(fn ConstructionScript
  (|CallParentFunction))