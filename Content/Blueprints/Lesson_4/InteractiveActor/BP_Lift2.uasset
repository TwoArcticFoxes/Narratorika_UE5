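; Interactive lift actor that, when triggered through a control interface, waits a set delay and then moves from its start location by an offset.
; A timeline with adjustable play rate lerps the position, optionally swapping endpoints to shuttle back and forth endlessly.
; Only the first trigger takes effect, and an optional chain flag calls Control on another actor as movement starts.
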(event Custom|StartMoving
  ;[1 1 1] StartMoving Event (Timeline)
  (Components|Timeline|SetPlayRate (Variables|Default|GetMovingTimeline) (/ (Variables|Default|GetPlayRate) (Variables|Default|GetPlayRateMod)))
  (bind _moving (Timeline|MovingTimeline PlayFromStart)
    (:Update
      (Transformation|SetActorLocation (Math|Vector|Lerp(Vector) (Variables|Default|GetStartLocatin) (Variables|Default|GetEndLocation) _moving) false false))
    (:Finished
      ;;[1 1 1] Repeat
      (if (Variables|Default|GetIsRepeat)
        (Variables|Default|SetTempLocation (Variables|Default|GetStartLocatin))
        (Variables|Default|SetStartLocatin (Variables|Default|GetEndLocation))
        (Variables|Default|SetEndLocation (Variables|Default|GetTempLocation))
        (CallFunction|StartMoving)))))

(event EventBeginPlay
  ;[1 1 1] Begin Play
  (|CallParentFunction)
  (bind _output_get (Variables|Default|SetStartLocatin (Transformation|GetActorLocation)))
  (Variables|Default|SetEndLocation (+ _output_get (Variables|Default|GetEndLocation))))

(event Collision|EventActorBeginOverlap
  (params (OtherActor :type Actor%20Object%20Reference))
  (|CallParentFunction OtherActor) ; This node is disabled and will not be called.\nDrag off pins to build functionality.
)

(event EventTick
  (params (DeltaSeconds :type Float%20%28single-precision%29))
  (|CallParentFunction DeltaSeconds) ; This node is disabled and will not be called.\nDrag off pins to build functionality.
)

(event EventControlInterface
  ;[1 1 1] Control
  (if (not (Variables|Default|GetIsMoved))
    (Variables|Default|SetIsMoved true)
    (Utilities|FlowControl|Delay (Variables|Default|GetDelay))
    (CallFunction|StartMoving)
    (if (Variables|Default|GetIsChain)
      (Default|Control (Variables|Default|GetControlActor)))))

(fn ConstructionScript
  (|CallParentFunction))