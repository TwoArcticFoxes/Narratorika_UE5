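; Hold-to-activate button that triggers its ControlActor when the third-person character stays inside its Sphere for TimeForWaiting.
; Entering swaps the Cylinder material and starts a one-shot timer, which calls Control on the linked actor and sets Done.
; Leaving before Done restores the material and clears the timer.
; Begin overlap ignores Done, so re-entering after activation triggers Control again after the wait.
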(event OnComponentBeginOverlap(Sphere)
  (params (OverlappedComponent :type Primitive%20Component%20Object%20Reference) (OtherActor :type Actor%20Object%20Reference) (OtherComp :type Primitive%20Component%20Object%20Reference) (OtherBodyIndex :type Integer) (bFromSweep :type Boolean) (SweepResult :type Hit%20Result%20Structure%20%28by%20ref%29))
  ;[1 1 1] Timer
  (Utilities|Casting|CastToBP_ThirdPersonCharacter OtherActor)
  (Rendering|Material|SetMaterial (Variables|Default|GetCylinder) 0 "/Game/LevelPrototyping/Materials/MI_PrototypeGrid_Rose_2.MI_PrototypeGrid_Rose_2")
  (bind _returnvalue (Utilities|Time|SetTimerbyEvent (delegate Custom|Waiting) (Variables|Default|GetTimeForWaiting))))

(event OnComponentEndOverlap(Sphere)
  (params (OverlappedComponent :type Primitive%20Component%20Object%20Reference) (OtherActor :type Actor%20Object%20Reference) (OtherComp :type Primitive%20Component%20Object%20Reference) (OtherBodyIndex :type Integer))
  ;[1 1 1] Timer
  (Utilities|Casting|CastToBP_ThirdPersonCharacter OtherActor)
  (if (not (Variables|Default|GetDone))
    (Rendering|Material|SetMaterial (Variables|Default|GetCylinder) 0 "/Game/LevelPrototyping/Materials/MI_PrototypeGrid_Rose.MI_PrototypeGrid_Rose")
    (Utilities|Time|ClearandInvalidateTimerbyHandle (stale OnComponentBeginOverlap(Sphere) _returnvalue))))

(event Custom|Waiting
  ;[1 1 1] Timer
  (Default|Control (Variables|Default|GetControlActor))
  (Variables|Default|SetDone true))

(event EventBeginPlay
  (|CallParentFunction) ; This node is disabled and will not be called.\nDrag off pins to build functionality.
)

(event Collision|EventActorBeginOverlap
  (params (OtherActor :type Actor%20Object%20Reference))
  (|CallParentFunction OtherActor) ; This node is disabled and will not be called.\nDrag off pins to build functionality.
)

(event EventTick
  (params (DeltaSeconds :type Float%20%28single-precision%29))
  (|CallParentFunction DeltaSeconds) ; This node is disabled and will not be called.\nDrag off pins to build functionality.
)

(fn ConstructionScript
  (|CallParentFunction))