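; BP_ButtonColorGold is an interactive button actor that changes its cylinder's material when interacted with.
; It extends a parent Blueprint, calling the parent BeginPlay before setting the cylinder to the Materials entry indexed by Color.
; The Interact event then swaps the cylinder to a fixed entry in the same Materials array, with no logic to revert it.
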(event EventBeginPlay
  ;[1 1 1] Color From Start
  (|CallParentFunction)
  (Rendering|Material|SetMaterial (Variables|Default|GetCylinder) 0 (Utilities|Array|Get(acopy) (Variables|Default|GetMaterials) (Variables|Default|GetColor))))

(event Collision|EventActorBeginOverlap
  (params (OtherActor :type Actor%20Object%20Reference))
  (|CallParentFunction OtherActor) ; This node is disabled and will not be called.\nDrag off pins to build functionality.
)

(event EventTick
  (params (DeltaSeconds :type Float%20%28single-precision%29))
  (|CallParentFunction DeltaSeconds) ; This node is disabled and will not be called.\nDrag off pins to build functionality.
)

(event EventInteract
  ;[1 1 1] Change Material
  (Rendering|Material|SetMaterial (Variables|Default|GetCylinder) 0 (Utilities|Array|Get(acopy) (Variables|Default|GetMaterials) 4)))

(fn ConstructionScript
  (|CallParentFunction))