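; BP_ButtonBlocked is an interactive button that stays blocked until another actor or trigger unlocks it through its Control event.
; Control waits for a configurable delay, swaps the Cylinder's material and opens a Gate node.
; Interact enters that gate and, when it is open, forwards a Control call to the linked ControlActor, so buttons and other controllable actors can be chained.
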(event EventBeginPlay
  (|CallParentFunction) ; This node is disabled and will not be called.\nDrag off pins to build functionality.
)

(event Collision|EventActorBeginOverlap
  (params (OtherActor :type Actor%20Object%20Reference))
  (|CallParentFunction OtherActor) ; This node is disabled and will not be called.\nDrag off pins to build functionality.
)

(event EventTick
  (params (DeltaSeconds :type Float%20%28single-precision%29))
  (|CallParentFunction DeltaSeconds) ; This node is disabled and will not be called.\nDrag off pins to build functionality.
)

(event EventControl
  (Utilities|FlowControl|Delay (Variables|Default|GetDelay))
  (Rendering|Material|SetMaterial (Variables|Default|GetCylinder) 0 (Variables|Default|GetMaterial))
  (Utilities|FlowControl|Gate true) ; enters at Open
)

(event EventInteract
  (Utilities|FlowControl|Gate true
    (:Exit
      (Default|Control (Variables|Default|GetControlActor)))))

(fn ConstructionScript
  (|CallParentFunction))