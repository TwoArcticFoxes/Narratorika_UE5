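; BP_Statue is a statue actor that flashes red and disappears when struck by something other than the player character.
; Its Capsule hit event ignores BP_ThirdPersonCharacter; any other actor swaps both SkeletalMesh materials to red Quinn variants, then destroys the statue after a short delay.
; The mesh's own hit event is empty, and an unconnected debug-print version of the same logic remains in the graph.
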(event OnComponentHit(SkeletalMesh)
  (params (HitComponent :type Primitive%20Component%20Object%20Reference) (OtherActor :type Actor%20Object%20Reference) (OtherComp :type Primitive%20Component%20Object%20Reference) (NormalImpulse :type Vector :default "0, 0, 0") (Hit :type Hit%20Result%20Structure%20%28by%20ref%29)))

(event OnComponentHit(Capsule)
  (params (HitComponent :type Primitive%20Component%20Object%20Reference) (OtherActor :type Actor%20Object%20Reference) (OtherComp :type Primitive%20Component%20Object%20Reference) (NormalImpulse :type Vector :default "0, 0, 0") (Hit :type Hit%20Result%20Structure%20%28by%20ref%29))
  (Utilities|Casting|CastToBP_ThirdPersonCharacter OtherActor
    (:CastFailed
      (Rendering|Material|SetMaterial (Variables|Default|GetSkeletalMesh) 0 "/Game/Characters/Mannequins/Materials/Instances/Quinn/MI_Quinn_01_Red.MI_Quinn_01_Red")
      (Rendering|Material|SetMaterial (Variables|Default|GetSkeletalMesh) 1 "/Game/Characters/Mannequins/Materials/Instances/Quinn/MI_Quinn_02_Red.MI_Quinn_02_Red")
      (Utilities|FlowControl|Delay 0.4)
      (Actor|DestroyActor))))

(event EventBeginPlay)

(event Collision|EventActorBeginOverlap
  (params (OtherActor :type Actor%20Object%20Reference)))

(event EventTick
  (params (DeltaSeconds :type Float%20%28single-precision%29)))

(fn ConstructionScript)