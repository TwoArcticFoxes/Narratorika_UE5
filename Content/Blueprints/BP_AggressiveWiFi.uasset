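; BP_AggressiveWiFi is an interactable two-cube actor that stops the bots' running state and triggers their aggressive call.
; Interacting clears BotsRun on BP_GameMode, then calls CallBotsAggressive.
; While BotsRun is set, trace hover or a scanner pulse applies a green overlay outline to both cubes.
; The pulse clears after a delay or on OutlineClose, with IsLight blocking overlapping pulses.
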(event EventBeginPlay
  ;[1 1 1] BeginPlay
  (|CallParentFunction))

(event Collision|EventActorBeginOverlap
  (params (OtherActor :type Actor%20Object%20Reference))
  (|CallParentFunction OtherActor) ; This node is disabled and will not be called.\nDrag off pins to build functionality.
)

(event EventTick
  (params (DeltaSeconds :type Float%20%28single-precision%29))
  (|CallParentFunction DeltaSeconds) ; This node is disabled and will not be called.\nDrag off pins to build functionality.
)

(event EventInteractInterface
  ;[1 1 1] StopBots
  (bind _asbp_game_mode (Utilities|Casting|CastToBP_GameMode (Game|GetGameMode)))
  (Variables|/Game/Blueprints/BP_GameMode.BP_GameMode_C|SetBotsRun _asbp_game_mode false)
  (Default|CallBotsAggressive _asbp_game_mode))

(event EventOutlineClose
  ;[1 1 1] Outline
  ;;[1 1 1] GameMode
  (Rendering|Material|SetOverlayMaterial (Variables|Default|GetCube) 0 :!class /Script/Engine.MeshComponent)
  (Rendering|Material|SetOverlayMaterial (Variables|Default|GetCube1) 0 :!class /Script/Engine.MeshComponent)
  (Variables|Default|SetIsLight false))

(event EventOutlineScannerOpen
  (params (Delay :type Float%20%28double-precision%29))
  ;[1 1 1] Outline
  ;;[1 1 1] GameMode
  (if (not (Variables|Default|GetIsLight))
    (bind _asbp_game_mode (Utilities|Casting|CastToBP_GameMode (Game|GetGameMode)))
    (if (Variables|/Game/Blueprints/BP_GameMode.BP_GameMode_C|GetBotsRun _asbp_game_mode)
      (Variables|Default|SetIsLight true)
      (Rendering|Material|SetOverlayMaterial (Variables|Default|GetCube) "/Game/Assets/Materials/My/MI_outlineGreen.MI_outlineGreen" :!class /Script/Engine.MeshComponent)
      (Rendering|Material|SetOverlayMaterial (Variables|Default|GetCube1) "/Game/Assets/Materials/My/MI_outlineGreen.MI_outlineGreen" :!class /Script/Engine.MeshComponent)
      (Utilities|FlowControl|Delay Delay)
      (Rendering|Material|SetOverlayMaterial (Variables|Default|GetCube) 0 :!class /Script/Engine.MeshComponent)
      (Rendering|Material|SetOverlayMaterial (Variables|Default|GetCube1) 0 :!class /Script/Engine.MeshComponent)
      (Variables|Default|SetIsLight false))))

(event EventOutlineInterface
  (params (Trace :type Boolean))
  ;[1 1 1] Outline
  ;;[1 1 1] Trace
  (if Trace
    (bind _asbp_game_mode (Utilities|Casting|CastToBP_GameMode (Game|GetGameMode)))
    (if (Variables|/Game/Blueprints/BP_GameMode.BP_GameMode_C|GetBotsRun _asbp_game_mode)
      (Rendering|Material|SetOverlayMaterial (Variables|Default|GetCube) "/Game/Assets/Materials/My/MI_outlineGreen.MI_outlineGreen" :!class /Script/Engine.MeshComponent)
      (Rendering|Material|SetOverlayMaterial (Variables|Default|GetCube1) "/Game/Assets/Materials/My/MI_outlineGreen.MI_outlineGreen" :!class /Script/Engine.MeshComponent))
    (else
      (Rendering|Material|SetOverlayMaterial (Variables|Default|GetCube) 0 :!class /Script/Engine.MeshComponent)
      (Rendering|Material|SetOverlayMaterial (Variables|Default|GetCube1) 0 :!class /Script/Engine.MeshComponent))))

(fn ConstructionScript
  (|CallParentFunction))