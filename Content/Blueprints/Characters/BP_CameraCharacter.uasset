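; BP_CameraCharacter is a possessable camera pawn that the player looks through with limited view angles.
; Possession rebuilds the HUD, adds the input mapping and applies pitch and yaw limits on the camera manager.
; HUD flags select normal, broken or one-time shutdown and glitch sequences, using BrokenAnim's delayed black-screen flashes.
; It also triggers scanner mode and shows a green overlay-material outline when traced or scanned.
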(event Custom|PossessCamera
  ;[1 1 1] PossessCamera
  (CallFunction|ClearWidgets)
  (bind _returnvalue (UserInterface|CreateWidget "/Game/UI/UMG_BlackScreen.UMG_BlackScreen_C"))
  (UserInterface|Viewport|AddtoViewport _returnvalue 0)
  (Variables|Default|SetBScreen _returnvalue)
  (Utilities|FlowControl|Sequence
    (:then_0
      (CallFunction|CreateHUD))
    (:then_1
      (CallFunction|SetInputs))
    (:then_2
      (CallFunction|SetCameraManager))))

(event Custom|Create%20HUD
  ;[1 1 1] HUD
  (if (Variables|HUD|GetIsNeedTurnOff)
    (if (not (Variables|HUD|GetIsTurnOff))
      ;;[1 1 1] Первое посещение сломанной камеры
      (Variables|HUD|SetIsTurnOff true)
      (bind _returnvalue (UserInterface|CreateWidget "/Game/UI/HUD/UMG_HUD_CameraCharacter.UMG_HUD_CameraCharacter_C"))
      (UserInterface|Viewport|AddtoViewport _returnvalue 0)
      (Utilities|BrokenAnim)
      (Widget|RemovefromParent _returnvalue))
    ;;[1 1 1] Второе посещение
    (bind _returnvalue_2 (UserInterface|CreateWidget "/Game/UI/HUD/UMG_HUD_BrokenCamera.UMG_HUD_BrokenCamera_C"))
    (UserInterface|Viewport|AddtoViewport _returnvalue_2 0)
    (Variables|Default|SetBrokenCameraHUD _returnvalue_2)
    (else
      ;;[1 1 1] Первое посещение взломанной камеры
      (if (Variables|HUD|GetIsNeedFix)
        (if (not (Variables|HUD|GetFixDone))
          (Variables|HUD|SetFixDone true)
          (bind _returnvalue_3 (UserInterface|CreateWidget "/Game/UI/HUD/UMG_HUD_CameraCharacter.UMG_HUD_CameraCharacter_C"))
          (UserInterface|Viewport|AddtoViewport _returnvalue_3 0)
          (Variables|Default|SetCameraHUD _returnvalue_3)
          (Utilities|BrokenAnim)
          (Utilities|FlowControl|Delay 1.0)
          (bind _returnvalue_4 (UserInterface|CreateWidget "/Game/UI/HUD/UMG_HUD_BrokenCamera.UMG_HUD_BrokenCamera_C"))
          (UserInterface|Viewport|AddtoViewport _returnvalue_4 0)
          (Utilities|FlowControl|Delay 1.0)
          (Widget|RemovefromParent _returnvalue_4)
          (Utilities|BrokenAnim)
          (else
            ;;[1 1 1] Второе посещение и нормальная камера
            (bind _returnvalue_5 (UserInterface|CreateWidget "/Game/UI/HUD/UMG_HUD_CameraCharacter.UMG_HUD_CameraCharacter_C" :!label _label))
            (UserInterface|Viewport|AddtoViewport _returnvalue_5 0)
            (Variables|Default|SetCameraHUD _returnvalue_5)))
        (else
          (goto _label))))))

(event Input|EnhancedActionEvents|EnhancedInputActionIA_Look
  (params (ActionValue :type Vector%202D%20Structure) (ElapsedSeconds :type Float%20%28double-precision%29) (TriggeredSeconds :type Float%20%28double-precision%29) (InputAction :type Input%20Action%20Object%20Reference :default "/Game/ThirdPerson/Input/Actions/IA_Look.IA_Look"))
  ;[1 1 1] Camera
  ;;[1 1 1] Mouse
  (:Triggered
    (Pawn|Input|AddControllerYawInput (.x ActionValue))
    (Pawn|Input|AddControllerPitchInput (.y ActionValue))))

(event Input|EnhancedActionEvents|EnhancedInputActionIA_Scanner
  (params (ActionValue :type Boolean) (ElapsedSeconds :type Float%20%28double-precision%29) (TriggeredSeconds :type Float%20%28double-precision%29) (InputAction :type Input%20Action%20Object%20Reference :default "/Game/ThirdPerson/Input/Actions/IA_Scanner.IA_Scanner"))
  ;[1 1 1] Scanner
  (:Started
    (Default|ScannerMode (Variables|Default|GetBP_Scanner) (Variables|Default|GetCamera) self)))

(event EventNeedPossess
  ;[1 1 1] Start
  (Pawn|Possess (Game|GetPlayerController 0) self)
  (CallFunction|PossessCamera))

(event EventClearWidgets
  (bind _brokencamerahud (Variables|Default|GetBrokenCameraHUD))
  (bind _camerahud (Variables|Default|GetCameraHUD))
  (bind _bscreen (Variables|Default|GetBScreen))
  ;[1 1 1] Clear Widgets
  (Utilities|FlowControl|Sequence
    (:then_0
      (Utilities|IsValid _brokencamerahud
        (:Is%20Valid
          (Widget|RemovefromParent _brokencamerahud))))
    (:then_1
      (Utilities|IsValid _camerahud
        (:Is%20Valid
          (Widget|RemovefromParent _camerahud))))
    (:then_2
      (Utilities|IsValid _bscreen
        (:Is%20Valid
          (Widget|RemovefromParent _bscreen))))))

(event EventOutlineInterface
  (params (Trace :type Boolean))
  ;[1 1 1] Outline
  (if Trace
    (Rendering|Material|SetOverlayMaterial (Variables|Default|GetCamer) "/Game/Assets/Materials/My/MI_outlineGreen.MI_outlineGreen" :!class /Script/Engine.MeshComponent)
    (else
      (Rendering|Material|SetOverlayMaterial (Variables|Default|GetCamer) 0 :!class /Script/Engine.MeshComponent))))

(event EventOutlineScannerOpen
  (params (Delay :type Float%20%28double-precision%29))
  ;[1 1 1] Outline
  (Rendering|Material|SetOverlayMaterial (Variables|Default|GetCamer) "/Game/Assets/Materials/My/MI_outlineGreen.MI_outlineGreen" :!class /Script/Engine.MeshComponent)
  (Utilities|FlowControl|Delay Delay)
  (Rendering|Material|SetOverlayMaterial (Variables|Default|GetCamer) 0 :!class /Script/Engine.MeshComponent))

(event EventOutlineClose
  ;[1 1 1] Outline
  (Rendering|Material|SetOverlayMaterial (Variables|Default|GetCamer) 0 :!class /Script/Engine.MeshComponent))

(fn ConstructionScript)

(fn SetCameraManager
  (bind _returnvalue (Game|GetPlayerCameraManager 0))
  (Variables|/Script/Engine.PlayerCameraManager|SetViewPitchMax _returnvalue 5.0)
  (Variables|/Script/Engine.PlayerCameraManager|SetViewYawMin _returnvalue (Variables|Default|GetView%20Yaw%20Min))
  (Variables|/Script/Engine.PlayerCameraManager|SetViewYawMax _returnvalue (Variables|Default|GetView%20Yaw%20Max)))

(fn SetInputs
  (bind _asplayer_controller (Utilities|Casting|CastToPlayerController (Pawn|GetController)))
  (Utilities|IsValid (PlayerController|LocalPlayerSubsystems|GetEnhancedInputLocalPlayerSubsystem _asplayer_controller)
    (:Is%20Valid
      (Input|AddMappingContext (PlayerController|LocalPlayerSubsystems|GetEnhancedInputLocalPlayerSubsystem _asplayer_controller) "/Game/ThirdPerson/Input/IMC_Default.IMC_Default" 0 "(bIgnoreAllPressedKeysUntilRelease=True,bForceImmediately=False)"))))

(fn CheckStatus
  (return (and (not (Variables|HUD|GetIsTurnOff)) (not (Variables|HUD|GetIsBroken)))))