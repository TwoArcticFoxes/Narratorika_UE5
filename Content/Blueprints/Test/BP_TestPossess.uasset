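; BP_TestPossess is a test interactable with a cube mesh that responds to light and interact interface events.
; LightInterface swaps the cube's material to a gold prototype grid.
; InteractInterface passes its HasElectricity value to a dispatcher on BP_GameInstance, then calls PossessCamera, stopping early if the game instance cast fails.
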(event EventBeginPlay
  (|CallParentFunction) ; This node is disabled and will not be called.\nDrag off pins to build functionality.
)

(event Collision|EventActorBeginOverlap
  (params (OtherActor :type Actor%20Object%20Reference))
  (|CallParentFunction OtherActor) ; This node is disabled and will not be called.\nDrag off pins to build functionality.
)

(event EventTick
  (params (DeltaSeconds :type Float%20%28single-precision%29))
  (|CallParentFunction DeltaSeconds) ; This node is disabled and will not be called.\nDrag off pins to build functionality.
)

(event EventLightInterface
  (Rendering|Material|SetMaterial (Variables|Default|GetCube) 0 "/Game/Assets/Props/Test/MI_PrototypeGrid_Gold.MI_PrototypeGrid_Gold"))

(event EventInteractInterface
  (bind _asbp_game_instance (Utilities|Casting|CastToBP_GameInstance (Game|GetGameInstance)))
  (Default|CallHasElectricityDis _asbp_game_instance (Variables|Default|GetHasElectricity))
  (Default|CallPossessCamera))

(fn ConstructionScript
  (|CallParentFunction))