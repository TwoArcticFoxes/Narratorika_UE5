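; Test Blueprint that starts a dialogue when interacted with through its InteractInterface event.
; The event creates a UMG_dialogue widget fed by the DT_StartDialogue table, adds it to the viewport and switches to UI-only input with the cursor shown.
; A PossessCamera callback bound to the widget removes it, restores game-only input, hides the cursor and calls the PossessCameraDialogue dispatcher.
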(event Custom|PossessCamera
  (bind _returnvalue (Game|GetPlayerController 0))
  ;[1 1 1] Create Widget Dialogue
  ;;[1 1 1] Delete
  (Utilities|FlowControl|Sequence
    (:then_0
      (Widget|RemovefromParent (stale EventInteractInterface _returnvalue_2))
      (Input|SetInputModeGameOnly _returnvalue false)
      (Variables|/Script/Engine.PlayerController|SetbShowMouseCursor _returnvalue false))
    (:then_1
      (Default|CallPossessCameraDialogue))))

(event EventInteractInterface
  (bind _returnvalue (Game|GetPlayerController 0))
  ;[1 1 1] Create Widget Dialogue
  ;;[1 1 1] Create
  (bind _returnvalue_2 (UserInterface|CreateWidget "/Game/UI/Start/UMG_dialogue.UMG_dialogue_C" _returnvalue "/Game/Blueprints/Tables/DT_StartDialogue.DT_StartDialogue"))
  (EventDispatchers|BindEventtoPossesCamera _returnvalue_2 (delegate Custom|PossessCamera))
  (UserInterface|Viewport|AddtoViewport _returnvalue_2 0)
  (Input|SetInputModeUIOnly _returnvalue 0 "DoNotLock" false)
  (Variables|/Script/Engine.PlayerController|SetbShowMouseCursor _returnvalue true))

(event Collision|EventActorBeginOverlap
  (params (OtherActor :type Actor%20Object%20Reference))
  (|CallParentFunction OtherActor) ; This node is disabled and will not be called.\nDrag off pins to build functionality.
)

(event EventTick
  (params (DeltaSeconds :type Float%20%28single-precision%29))
  (|CallParentFunction DeltaSeconds) ; This node is disabled and will not be called.\nDrag off pins to build functionality.
)

(event EventBeginPlay
  (|CallParentFunction) ; This node is disabled and will not be called.\nDrag off pins to build functionality.
)

(fn ConstructionScript
  (|CallParentFunction))