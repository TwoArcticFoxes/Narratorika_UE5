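; BP_CameraCharacter is a player character Blueprint whose only live logic is camera look through Enhanced Input.
; IA_Look feeds its X and Y values into controller yaw and pitch.
; A disconnected setup chain, which never runs, would create the UMG_HUD_CameraCharacter widget, show the mouse cursor, toggle PostProcess off then on, and register the IMC_Default mapping context.
; The construction script is empty.
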(event Input|EnhancedActionEvents|EnhancedInputActionIA_Look
  (params (ActionValue :type Vector%202D%20Structure) (ElapsedSeconds :type Float%20%28double-precision%29) (TriggeredSeconds :type Float%20%28double-precision%29) (InputAction :type Input%20Action%20Object%20Reference :default "/Game/ThirdPerson/Input/Actions/IA_Look.IA_Look"))
  ;[1 1 1] Camera
  ;;[1 1 1] Mouse
  (:Triggered
    (Pawn|Input|AddControllerYawInput (.x ActionValue))
    (Pawn|Input|AddControllerPitchInput (.y ActionValue))))

(fn ConstructionScript)