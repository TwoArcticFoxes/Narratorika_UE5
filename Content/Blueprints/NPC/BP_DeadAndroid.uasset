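; BP_DeadAndroid is a dead android that can be highlighted and described when traced.
; Outline interface events set a red overlay material on the skeletal mesh and start a hint while traced, then clear the overlay when the trace ends or the outline closes.
; A scanner event shows the same outline for a supplied delay before clearing it.
; Description events pass the trace state and text to a description object.
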(event EventObjectDescription
  (params (Trace :type Boolean))
  (Default|Description (Variables|Default|GetBP_descriptionobject) Trace (Variables|Default|GetDescriptionText)))

(event EventOutlineScannerOpen
  (params (Delay :type Float%20%28double-precision%29))
  ;[1 1 1] Outline
  (Rendering|Material|SetOverlayMaterial (Variables|Default|GetSkeletalMesh) "/Game/Assets/Materials/My/MI_outlineRed.MI_outlineRed" :!class /Script/Engine.MeshComponent)
  (Utilities|FlowControl|Delay Delay)
  (Rendering|Material|SetOverlayMaterial (Variables|Default|GetSkeletalMesh) 0 :!class /Script/Engine.MeshComponent))

(event EventOutlineInterface
  (params (Trace :type Boolean))
  ;[1 1 1] Outline
  (if Trace
    (Rendering|Material|SetOverlayMaterial (Variables|Default|GetSkeletalMesh) "/Game/Assets/Materials/My/MI_outlineRed.MI_outlineRed" :!class /Script/Engine.MeshComponent)
    (Default|StartHint (Variables|Default|GetHint))
    (else
      (Rendering|Material|SetOverlayMaterial (Variables|Default|GetSkeletalMesh) 0 :!class /Script/Engine.MeshComponent))))

(event EventOutlineClose
  ;[1 1 1] Outline
  (Rendering|Material|SetOverlayMaterial (Variables|Default|GetSkeletalMesh) 0 :!class /Script/Engine.MeshComponent))

(fn ConstructionScript)