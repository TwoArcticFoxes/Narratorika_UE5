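; BP_AggressiveCleaner is a knife-fitted cleaner robot NPC that escalates to security when it repeatedly bumps the player.
; Player overlaps with its Box increment a shared GameMode Collision counter, which calls security about bots once past its limit.
; Trace and scanner interface events toggle a red overlay-material outline on body and knives, with the scanner outline timing out.
; A looping AIMoveTo patrol exists but is disabled, as nothing calls it.
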(event OnComponentBeginOverlap(Box)
  (params (OverlappedComponent :type Primitive%20Component%20Object%20Reference) (OtherActor :type Actor%20Object%20Reference) (OtherComp :type Primitive%20Component%20Object%20Reference) (OtherBodyIndex :type Integer) (bFromSweep :type Boolean) (SweepResult :type Hit%20Result%20Structure%20%28by%20ref%29))
  (bind _returnvalue (Game|GetGameMode))
  (bind _asbp_game_mode (Utilities|Casting|CastToBP_GameMode _returnvalue))
  (bind _collision (Variables|/Game/Blueprints/BP_GameMode.BP_GameMode_C|GetCollision _asbp_game_mode))
  ;[1 1 1] Hit Player
  (if (== OtherActor (Game|GetPlayerCharacter 0))
    (if (<= _collision 5)
      (Math|Integer|IncrementInt _collision)
      (else
        (Default|CallSecurityAboutBots _asbp_game_mode)))))

(event Custom|Patrol
  ;[1 0.0666 0] ОТКЛЮЧЕНО
  ;;[1 1 1] Patrol
  (AI|AIMoveTo self (.RandomLocation (AI|Navigation|GetRandomReachablePointinRadius (Transformation|GetActorLocation) 7e+02 0 0)) (Utilities|Array|Get(acopy) (Variables|Default|GetPatrolPoints) (Variables|Default|GetIndex)) 2e+01 false
    (:OnSuccess
      _)
    (:OnFail
      _))
  (bind _result (Math|Integer|IncrementInt (Variables|Default|GetIndex))
    (:%20%20
      (Variables|Default|SetIndex (Math|Integer|%(Integer) _result (Utilities|Array|Length (Variables|Default|GetPatrolPoints))))
      (Utilities|FlowControl|Delay (Math|Random|RandomFloatinRange 0.5 3.0))
      (CallFunction|Patrol))))

(event EventOutlineInterface
  (params (Trace :type Boolean))
  ;[1 1 1] Light
  ;;[1 1 1] Trace
  (if Trace
    (CallFunction|SetOutline)
    (else
      (CallFunction|EndOutline))))

(event EventBeginPlay
  ;[1 0.0666 0] ОТКЛЮЧЕНО
  ;;[1 1 1] Begin play
)

(event EventOutlineScannerOpen
  (params (Delay :type Float%20%28double-precision%29))
  ;[1 1 1] Light
  ;;[1 1 1] GameMode
  (CallFunction|SetOutline)
  (Utilities|FlowControl|Delay 5.0)
  (CallFunction|EndOutline))

(event EventOutlineClose
  ;[1 1 1] Light
  ;;[1 1 1] GameMode
  (CallFunction|EndOutline))

(event EventObjectDescription
  (params (Trace :type Boolean)))

(fn ConstructionScript)

(fn SetOutline
  (if (not (Variables|Default|GetExist))
    (Variables|Default|SetExist true)
    (Utilities|FlowControl|Sequence
      (:then_0
        (Rendering|Material|SetOverlayMaterial (Variables|Default|GetRobotBody) "/Game/Assets/Materials/My/MI_outlineRed.MI_outlineRed" :!class /Script/Engine.MeshComponent))
      (:then_1
        (Rendering|Material|SetOverlayMaterial (Variables|Default|GetSM_Knife_03) "/Game/Assets/Materials/My/MI_outlineRed.MI_outlineRed" :!class /Script/Engine.MeshComponent))
      (:then_2
        (Rendering|Material|SetOverlayMaterial (Variables|Default|GetSM_Knife_04) "/Game/Assets/Materials/My/MI_outlineRed.MI_outlineRed" :!class /Script/Engine.MeshComponent))
      (:then_3
        (Rendering|Material|SetOverlayMaterial (Variables|Default|GetSM_Knife_05) "/Game/Assets/Materials/My/MI_outlineRed.MI_outlineRed" :!class /Script/Engine.MeshComponent))
      (:then_4
        (Rendering|Material|SetOverlayMaterial (Variables|Default|GetSM_Knife_06) "/Game/Assets/Materials/My/MI_outlineRed.MI_outlineRed" :!class /Script/Engine.MeshComponent)))))

(fn EndOutline
  (Utilities|FlowControl|Sequence
    (:then_0
      (Rendering|Material|SetOverlayMaterial (Variables|Default|GetRobotBody) 0 :!class /Script/Engine.MeshComponent))
    (:then_1
      (Rendering|Material|SetOverlayMaterial (Variables|Default|GetSM_Knife_03) 0 :!class /Script/Engine.MeshComponent))
    (:then_2
      (Rendering|Material|SetOverlayMaterial (Variables|Default|GetSM_Knife_04) 0 :!class /Script/Engine.MeshComponent))
    (:then_3
      (Rendering|Material|SetOverlayMaterial (Variables|Default|GetSM_Knife_05) 0 :!class /Script/Engine.MeshComponent))
    (:then_4
      (Rendering|Material|SetOverlayMaterial (Variables|Default|GetSM_Knife_06) 0 :!class /Script/Engine.MeshComponent)
      (Variables|Default|SetExist false))))