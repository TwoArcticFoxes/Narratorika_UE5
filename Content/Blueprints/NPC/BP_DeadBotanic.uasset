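; Dead gardener android NPC that serves as the armor pickup in the quest progression.
; Interacting during the NeedArmor stage plays sounds, and on first success swaps two body materials, shows a hint and advances GameMode progress to HaveArmor.
; Outline interface events apply a yellow, green or red overlay material by PlayerProgress, with stage hints when traced.
; Description events likewise choose the name and action prompt by progress and pass them to BPDescriptionobject.
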(event EventBeginPlay)

(event Collision|EventActorBeginOverlap
  (params (OtherActor :type Actor%20Object%20Reference)))

(event EventTick
  (params (DeltaSeconds :type Float%20%28single-precision%29)))

(event EventOutlineScannerOpen
  (params (Delay :type Float%20%28double-precision%29))
  ;[1 1 1] Outline
  (CallFunction|SetOutline false)
  (Utilities|FlowControl|Delay Delay)
  (Rendering|Material|SetOverlayMaterial (Variables|Default|GetSkeletalMesh) 0 :!class /Script/Engine.MeshComponent))

(event EventOutlineInterface
  (params (Trace :type Boolean))
  ;[1 1 1] Outline
  (if Trace
    (CallFunction|SetOutline Trace)
    (else
      (Rendering|Material|SetOverlayMaterial (Variables|Default|GetSkeletalMesh) 0 :!class /Script/Engine.MeshComponent))))

(event EventOutlineClose
  ;[1 1 1] Outline
  (Rendering|Material|SetOverlayMaterial (Variables|Default|GetSkeletalMesh) 0 :!class /Script/Engine.MeshComponent))

(event EventInteractInterface
  (bind _returnvalue (Game|GetGameMode))
  (bind _asbp_game_mode (Utilities|Casting|CastToBP_GameMode _returnvalue))
  ;[1 1 1] Interact
  (if (Utilities|Enum|Equal(Enum) (Variables|/Game/Blueprints/BP_GameMode.BP_GameMode_C|GetPlayerProgress _asbp_game_mode) "NewEnumerator1")
    (Audio|PlaySoundatLocation "/Game/Assets/Audio/Sounds/Wave/push.push" (Transformation|GetActorLocation) "0, 0, 0" 1.0 1.0 0.0 0 0 0 0)
    (if (Variables|Default|GetBotArmored)
      (Variables|Default|SetBotArmored false)
      (Utilities|FlowControl|Delay 0.7)
      (Audio|PlaySoundatLocation "/Game/Assets/Audio/Sounds/Wave/take.take" (Transformation|GetActorLocation) "0, 0, 0" 1.0 1.0 0.0 0 0 0 0)
      (CallFunction|Hint 3)
      (Rendering|Material|SetMaterial (Variables|Default|GetSkeletalMesh) 0 "/Game/Assets/Materials/Materials/Instances/Quinn/MI_Quinn_DarkGreen_01.MI_Quinn_DarkGreen_01")
      (Rendering|Material|SetMaterial (Variables|Default|GetSkeletalMesh) 1 "/Game/Assets/Materials/Materials/Instances/Quinn/MI_Quinn_DarkGreen_02.MI_Quinn_DarkGreen_02")
      (Utilities|FlowControl|Delay 1.0)
      (Default|CallNewProgress _asbp_game_mode "NewEnumerator2")
      (else
        (CallFunction|Hint 2)))))

(event EventObjectDescription
  (params (Trace :type Boolean))
  ;[1 1 1] Description
  (switch Utilities|FlowControl|Switch|SwitchonE_playerProgress (Variables|/Game/Blueprints/BP_GameMode.BP_GameMode_C|GetPlayerProgress (.AsBP%20Game%20Mode (Utilities|Casting|CastToBP_GameMode (Game|GetGameMode))))
    (:NewEnumerator5
      (Variables|Default|SetText "Укрепленный андроид-садовник" :!label _label))
    (:NewEnumerator6
      (goto _label))
    (:NewEnumerator4
      (goto _label))
    (:NewEnumerator0
      (goto _label))
    (:NewEnumerator9
      (goto _label))
    (:NewEnumerator1
      (goto _label))
    (:NewEnumerator2
      (Variables|Default|SetText "Андроид-садовник" :!label _label_2))
    (:NewEnumerator3
      (goto _label_2))
    (:NewEnumerator7
      (goto _label_2))
    (:NewEnumerator8
      (goto _label_2)))
  (Default|Description (Variables|Default|GetBP_descriptionobject) Trace (Variables|Default|GetText)))

(event EventObjectActionDescription
  (params (Trace :type Boolean))
  ;[1 1 1] Description
  (switch Utilities|FlowControl|Switch|SwitchonE_playerProgress (Variables|/Game/Blueprints/BP_GameMode.BP_GameMode_C|GetPlayerProgress (.AsBP%20Game%20Mode (Utilities|Casting|CastToBP_GameMode (Game|GetGameMode))))
    (:NewEnumerator5
      (Variables|Default|SetAction%20Descr%20Text "" :!label _label))
    (:NewEnumerator6
      (goto _label))
    (:NewEnumerator4
      (goto _label))
    (:NewEnumerator0
      (goto _label))
    (:NewEnumerator9
      (goto _label))
    (:NewEnumerator1
      (Variables|Default|SetAction%20Descr%20Text " <BoldH>[Е] Изучить </>"))
    (:NewEnumerator2
      (goto _label))
    (:NewEnumerator3
      (goto _label))
    (:NewEnumerator7
      (goto _label))
    (:NewEnumerator8
      (goto _label)))
  (Default|ActionDescripton (Variables|Default|GetBP_descriptionobject) Trace (Variables|Default|GetAction%20Descr%20Text)))

(fn ConstructionScript)

(fn SetOutline
  (params (Trace :type Boolean))
  (Variables|Default|SetTrace Trace)
  (switch Utilities|FlowControl|Switch|SwitchonE_playerProgress (Variables|/Game/Blueprints/BP_GameMode.BP_GameMode_C|GetPlayerProgress (.AsBP%20Game%20Mode (Utilities|Casting|CastToBP_GameMode (Game|GetGameMode))))
    (:NewEnumerator5
      (Rendering|Material|SetOverlayMaterial (Variables|Default|GetSkeletalMesh) "/Game/Assets/Materials/My/MI_outlineYe.MI_outlineYe" :!class /Script/Engine.MeshComponent :!label _label)
      (if (Variables|Default|GetTrace)
        (CallFunction|Hint)))
    (:NewEnumerator6
      (goto _label))
    (:NewEnumerator4
      (goto _label))
    (:NewEnumerator0
      (goto _label))
    (:NewEnumerator9
      (goto _label))
    (:NewEnumerator1
      (Rendering|Material|SetOverlayMaterial (Variables|Default|GetSkeletalMesh) "/Game/Assets/Materials/My/MI_outlineGreen.MI_outlineGreen" :!class /Script/Engine.MeshComponent)
      (if (Variables|Default|GetTrace)
        (CallFunction|Hint 1)))
    (:NewEnumerator2
      (Rendering|Material|SetOverlayMaterial (Variables|Default|GetSkeletalMesh) "/Game/Assets/Materials/My/MI_outlineRed.MI_outlineRed" :!class /Script/Engine.MeshComponent :!label _label_2))
    (:NewEnumerator3
      (goto _label_2))
    (:NewEnumerator7
      (goto _label_2))
    (:NewEnumerator8
      (goto _label_2))))

(fn Hint
  (params (ID :type Integer))
  (Default|StartHint (Utilities|Array|Get(acopy) (Variables|Default|GetBP_hint) ID)))