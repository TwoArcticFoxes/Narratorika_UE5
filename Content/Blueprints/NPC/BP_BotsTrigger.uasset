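; BP_BotsTrigger is a one-shot trigger that launches the aggressive cleaner bot when its StartHint event runs.
; A Launched flag lets it fire once, then it finds a single BP_AggressiveCleaner through GetActorOfClass.
; It casts that actor's AI controller to AggressiveCleaerControler and sets the "launched" Blackboard key to true.
; IsNeed always returns false.
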(event EventStartHint
  (if (not (Variables|Default|Getlaunched))
    (Variables|Default|Setlaunched true)
    (bind _returnvalue (Actor|GetActorOfClass "/Game/Blueprints/NPC/BP_AggressiveCleaner.BP_AggressiveCleaner_C"))
    (bind _asaggressive_cleaer_controler (Utilities|Casting|CastToAggressiveCleaerControler (AI|GetAIController _returnvalue)))
    (AI|Components|Blackboard|SetValueasBool (Variables|/Script/AIModule.AIController|GetBlackboard _asaggressive_cleaer_controler) (Utilities|Name|MakeLiteralName "launched") true)))

(fn ConstructionScript)

(fn IsNeed
  (return false))