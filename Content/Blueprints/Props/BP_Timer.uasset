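; BP_Timer is an interactable timer button prop that triggers a linked ControlActor through ControlInterface after a countdown.
; Interacting starts a looping one-second countdown, blocks re-triggering while in process, and resets a few seconds after firing.
; Its W_TimerButton widget receives a reference to the actor on BeginPlay.
; Trace and scanner events drive an overlay-material outline colored by state, and the press prompt hides while running.
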(event Custom|Countdown
  ;[1 1 1] Interact
  (Math|Float|IncrementFloat (Variables|Default|GetCountdownProgress)
    (:%20%20
      (if (== (Variables|Default|GetCountdownDuration) (Variables|Default|GetCountdownProgress))
        (Utilities|FlowControl|Delay 0.2)
        (Default|ControlInterface (Variables|Default|GetControlActor))
        (Utilities|FlowControl|Delay 5.0)
        (Utilities|Time|ClearandInvalidateTimerbyHandle (Variables|Default|GetTimer))
        (Variables|Default|SetCountdownProgress 0.0)
        (Variables|Default|SetInProcess false)))))

(event EventBeginPlay
  ;[1 1 1] Widget
  (|CallParentFunction)
  (bind _asw_timer_button (Utilities|Casting|CastToW_TimerButton (UserInterface|GetUserWidgetObject (Variables|Default|GetWidget))))
  (Variables|/Game/UI/BPWidgets/W_TimerButton.W_TimerButton_C|SetTimerButtonRef _asw_timer_button self))

(event Collision|EventActorBeginOverlap
  (params (OtherActor :type Actor%20Object%20Reference))
  (|CallParentFunction OtherActor) ; This node is disabled and will not be called.\nDrag off pins to build functionality.
)

(event EventTick
  (params (DeltaSeconds :type Float%20%28single-precision%29))
  (|CallParentFunction DeltaSeconds) ; This node is disabled and will not be called.\nDrag off pins to build functionality.
)

(event EventInteractInterface
  ;[1 1 1] Interact
  (if (not (Variables|Default|GetInProcess))
    (Variables|Default|SetInProcess true)
    (bind _returnvalue (Utilities|Time|SetTimerbyEvent (delegate Custom|Countdown) 1.0 true))
    (Variables|Default|SetTimer _returnvalue)))

(event EventOutlineInterface
  (params (Trace :type Boolean))
  ;[1 1 1] Outline
  (if Trace
    (CallFunction|SetOutline)
    (else
      (Rendering|Material|SetOverlayMaterial (Variables|Default|GetSphere1) 0 :!class /Script/Engine.MeshComponent))))

(event EventOutlineScannerOpen
  (params (Delay :type Float%20%28double-precision%29))
  ;[1 1 1] Outline
  (CallFunction|SetOutline)
  (Utilities|FlowControl|Delay Delay)
  (Rendering|Material|SetOverlayMaterial (Variables|Default|GetSphere1) 0 :!class /Script/Engine.MeshComponent))

(event EventOutlineClose
  ;[1 1 1] Outline
  (Rendering|Material|SetOverlayMaterial (Variables|Default|GetSphere1) 0 :!class /Script/Engine.MeshComponent))

(event EventObjectActionDescription
  (params (Trace :type Boolean))
  ;[1 1 1] Description
  (if (Variables|Default|GetInProcess)
    (Variables|Default|SetAction%20Descr%20Text_0 "     ")
    (else
      (Variables|Default|SetAction%20Descr%20Text_0 " <BoldH>[Е] Нажать </>")))
  (Default|ActionDescripton (Variables|Default|GetBP_descriptionobject) Trace (Variables|Default|GetAction%20Descr%20Text_0)))

(fn ConstructionScript
  (|CallParentFunction))

(fn SetOutline
  (if (Variables|Default|GetInProcess)
    (Rendering|Material|SetOverlayMaterial (Variables|Default|GetSphere1) "/Game/Assets/Materials/My/MI_outlineYe.MI_outlineYe" :!class /Script/Engine.MeshComponent)
    (else
      (Rendering|Material|SetOverlayMaterial (Variables|Default|GetSphere1) "/Game/Assets/Materials/My/MI_outlineGreen.MI_outlineGreen" :!class /Script/Engine.MeshComponent))))