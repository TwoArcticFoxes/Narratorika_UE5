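; BP_BrokenCamera is a broken CCTV camera prop that the player can highlight and inspect.
; Outline events set or clear a red overlay material on the camera mesh: a trace also starts its hint, while a scanner reveal clears after a delay.
; The description event passes a hardcoded Russian "Broken camera" label to a description object.
; IsNeed always returns false, and construction and default events are empty.
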(event EventBeginPlay)

(event Collision|EventActorBeginOverlap
  (params (OtherActor :type Actor%20Object%20Reference)))

(event EventTick
  (params (DeltaSeconds :type Float%20%28single-precision%29)))

(event EventOutlineClose
  (Rendering|Material|SetOverlayMaterial (Variables|Default|GetSM_CCTV_Camera) 0 :!class /Script/Engine.MeshComponent))

(event EventOutlineScannerOpen
  (params (Delay :type Float%20%28double-precision%29))
  (Rendering|Material|SetOverlayMaterial (Variables|Default|GetSM_CCTV_Camera) "/Game/Assets/Materials/My/MI_outlineRed.MI_outlineRed" :!class /Script/Engine.MeshComponent)
  (Utilities|FlowControl|Delay Delay)
  (Rendering|Material|SetOverlayMaterial (Variables|Default|GetSM_CCTV_Camera) 0 :!class /Script/Engine.MeshComponent))

(event EventOutlineInterface
  (params (Trace :type Boolean))
  (if Trace
    (Rendering|Material|SetOverlayMaterial (Variables|Default|GetSM_CCTV_Camera) "/Game/Assets/Materials/My/MI_outlineRed.MI_outlineRed" :!class /Script/Engine.MeshComponent)
    (Default|StartHint (Variables|Default|GetHint))
    (else
      (Rendering|Material|SetOverlayMaterial (Variables|Default|GetSM_CCTV_Camera) 0 :!class /Script/Engine.MeshComponent))))

(event EventObjectDescription
  (params (Trace :type Boolean))
  (Default|Description (Variables|Default|GetBP_descriptionobject) Trace "Сломанная камера"))

(fn ConstructionScript)

(fn IsNeed
  (return false))