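; Shelf prop that fills three levels (lower, middle, top) with boxes at construction time, using instanced mesh components.
; Each level's layout comes from its stat property or, with Random enabled, a random roll.
; SetOneShelf builds a two-box stack, a single box or a row of three from the Box01–Box04 array.
; Each box gets slight position and yaw jitter.
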(event EventBeginPlay)

(event Collision|EventActorBeginOverlap
  (params (OtherActor :type Actor%20Object%20Reference)))

(event EventTick
  (params (DeltaSeconds :type Float%20%28single-precision%29)))

(fn ConstructionScript
  (bind _returnvalue (Math|Random|RandomIntegerinRange 0 3))
  (bind _returnvalue_2 (Math|Conversions|ToByte(Integer) _returnvalue))
  (bind _returnvalue_3 (Utilities|Enum|ByteToEnumE_Shelf _returnvalue_2))
  (CallFunction|SetBoxArray)
  (Components|InstancedStaticMesh|AddInstance (Variables|Default|GetShelf) (Math|Transform|MakeTransform "0, 0, 0") false)
  (if (Variables|Default|GetRandom)
    (bind _output_get (Variables|Default|SetLowerStat _returnvalue_3))
    (CallFunction|SetOneShelf (Variables|Default|GetLowerLocation) _output_get)
    (CallFunction|SetOneShelf (Variables|Default|GetMiddleLocation) _returnvalue_3)
    (CallFunction|SetOneShelf (Variables|Default|GetTopLocation) _returnvalue_3)
    (else
      (CallFunction|SetOneShelf (Variables|Default|GetLowerLocation) (Variables|Default|GetLowerStat))
      (CallFunction|SetOneShelf (Variables|Default|GetMiddleLocation) (Variables|Default|GetMiddleStat))
      (CallFunction|SetOneShelf (Variables|Default|GetTopLocation) (Variables|Default|GetTopStat)))))

(fn Transform
  (params (InVec :type Vector))
  (bind (_x _y _z) (Math|Vector|BreakVector InVec))
  (return (Math|Transform|MakeTransform (Math|Vector|MakeVector (+ (Math|Random|RandomFloatinRange -15.0 15.0) _x) (+ _y (Math|Random|RandomFloatinRange -5.0 5.0)) _z) (Math|Rotator|MakeRotator 0.0 0.0 (Math|Random|RandomFloatinRange 1e+01 -1e+01)))))

(fn SetBoxArray
  (bind _boxarray (Variables|Default|GetBoxArray))
  (Utilities|Array|SetArrayElem _boxarray 0 (Variables|Default|GetBox_01) true)
  (Utilities|Array|SetArrayElem _boxarray 1 (Variables|Default|GetBox_02) true)
  (Utilities|Array|SetArrayElem _boxarray 2 (Variables|Default|GetBox_03) true)
  (Utilities|Array|SetArrayElem _boxarray 3 (Variables|Default|GetBox_04)))

(fn TransformandSet
  (params (self2 :type Instanced%20Static%20Mesh%20Component%20Object%20Reference) (InVec :type Vector))
  (bind _returnvalue (CallFunction|Transform InVec))
  (Components|InstancedStaticMesh|AddInstance self2 _returnvalue false))

(fn SetOneShelf
  (params (Location :type Vector) (Stat :type E_Shelf%20Enum :default "NewEnumerator0"))
  (bind _returnvalue (Math|Random|RandomIntegerinRange 1 3))
  (bind _boxarray (Variables|Default|GetBoxArray))
  (bind _output (Utilities|Array|Get(acopy) _boxarray _returnvalue))
  (Variables|Default|SetLocation Location)
  (switch Utilities|FlowControl|Switch|SwitchonE_Shelf Stat
    (:NewEnumerator0
      (CallFunction|TransformandSet (Variables|Default|GetBox_01) (Variables|Default|GetLocation))
      (CallFunction|TransformandSet (Utilities|Array|Get(acopy) (Variables|Default|GetBoxArray) (Math|Random|RandomIntegerinRange 0 1)) (Math|Vector|MakeVector (.x (Variables|Default|GetLocation)) (.y (Variables|Default|GetLocation)) (+ (.z (Variables|Default|GetLocation)) 42.0))))
    (:NewEnumerator1
      (CallFunction|TransformandSet (Utilities|Array|Get(acopy) (Variables|Default|GetBoxArray) (Math|Random|RandomIntegerinRange 0 3)) (Math|Vector|MakeVector (+ (.x (Variables|Default|GetLocation)) (Math|Random|RandomFloatinRange -7e+01 7e+01)) (+ (.y (Variables|Default|GetLocation)) (Math|Random|RandomFloatinRange -1e+01 1e+01)) (.z (Variables|Default|GetLocation)))))
    (:NewEnumerator2
      (CallFunction|TransformandSet _output (Variables|Default|GetLocation))
      (CallFunction|TransformandSet _output (Math|Vector|MakeVector (+ (.x (Variables|Default|GetLocation)) -7e+01) (.y (Variables|Default|GetLocation)) (.z (Variables|Default|GetLocation))))
      (CallFunction|TransformandSet _output (Math|Vector|MakeVector (+ (.x (Variables|Default|GetLocation)) 7e+01) (.y (Variables|Default|GetLocation)) (.z (Variables|Default|GetLocation)))))))