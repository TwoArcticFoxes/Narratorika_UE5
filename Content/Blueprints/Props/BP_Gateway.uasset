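; Gateway prop with three swinging doors (inside, middle-outside, outside), triggered by ID through ControlInterface and locked against re-triggering while moving.
; BeginPlay caches start and end transforms per door; a timeline lerps the active door between them, then ResetVars swaps them and toggles its closed state.
; СheckFunction chains moves so an open inside or outside door closes before the opposite opens, with the middle door always following the outside one.
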(event Custom|DoorMove
  (params (DoorID :type Integer))
  ;[1 1 1] Moving
  (Variables|Vars|SetActiveDoorID DoorID)
  (CallFunction|СheckFunction (Variables|Vars|GetActiveDoorID))
  (bind _activedoor (CallFunction|SetActiveDoorVars))
  (Audio|PlaySoundatLocation "/Game/Assets/Audio/Sounds/SC_DoorSound_02.SC_DoorSound_02" (Transformation|GetWorldLocation _activedoor) "0, 0, 0" 1.0 1.0 0.0 0 0 0 0)
  (bind _moving (Timeline|TL_MovingDoor PlayFromStart)
    (:Update
      (CallFunction|Rotation _moving))
    (:Finished
      (CallFunction|ResetVars (Variables|Vars|GetActiveDoorID)))))

(event EventBeginPlay
  ;[1 1 1] Set start parameters
  (|CallParentFunction)
  (CallFunction|SetVars (Variables|Default|GetDoor_01_Inside))
  (CallFunction|SetVars (Variables|Default|GetDoor_02_MediumOutside) 1)
  (CallFunction|SetVars (Variables|Default|GetDoor_03_Outside) 2))

(event Collision|EventActorBeginOverlap
  (params (OtherActor :type Actor%20Object%20Reference))
  (|CallParentFunction OtherActor) ; This node is disabled and will not be called.\nDrag off pins to build functionality.
)

(event EventTick
  (params (DeltaSeconds :type Float%20%28single-precision%29))
  (|CallParentFunction DeltaSeconds) ; This node is disabled and will not be called.\nDrag off pins to build functionality.
)

(event EventControlInterface
  (params (ID :type Integer))
  ;[1 1 1] Moving
  (if (not (Variables|Default|GetIsMoving))
    (Variables|Default|SetIsMoving true)
    (Variables|Vars|SetActiveDoorID ID)
    (CallFunction|СheckFunction (Variables|Vars|GetActiveDoorID))
    (bind _activedoor (CallFunction|SetActiveDoorVars))
    (Audio|PlaySoundatLocation "/Game/Assets/Audio/Sounds/SC_DoorSound_02.SC_DoorSound_02" (Transformation|GetWorldLocation _activedoor) "0, 0, 0" 1.0 1.0 0.0 0 0 0 0)
    (bind _moving (Timeline|TL_MovingDoor PlayFromStart)
      (:Update
        (CallFunction|Rotation _moving))
      (:Finished
        (CallFunction|ResetVars (Variables|Vars|GetActiveDoorID))))))

(fn ConstructionScript
  (|CallParentFunction))

(fn SetVars
  (params (StaticMesh :type Static%20Mesh%20Component%20Object%20Reference) (ID :type Integer))
  (bind _output_get (LocalVariables|SetL_lID ID))
  (Utilities|FlowControl|Sequence
    (:then_0
      (bind _output_get_2 (LocalVariables|SetL_StartLocation (Transformation|GetWorldLocation StaticMesh)))
      (Utilities|Array|SetArrayElem (Variables|Vars|GetStartLocationArray) _output_get _output_get_2)
      (switch int _output_get
        (:0
          (LocalVariables|SetL_EndLocation (+ _output_get_2 "-3.000000,-15.000000,0.000000") :!label _label))
        (:1
          (goto _label))
        (:2
          (LocalVariables|SetL_EndLocation (+ _output_get_2 "-3.000000,15.000000,0.000000"))))
      (Utilities|Array|SetArrayElem (Variables|Vars|GetEndLocationArray) _output_get (LocalVariables|GetL_EndLocation)))
    (:then_1
      (bind _output_get_3 (Variables|Vars|SetStartRotation (Transformation|GetWorldRotation StaticMesh)))
      (Utilities|Array|SetArrayElem (Variables|Vars|GetStartRotationArray) _output_get _output_get_3)
      (Variables|Vars|SetEndRotation (Math|Rotator|CombineRotators _output_get_3 "0.000000,90.000000,0.000000"))
      (Utilities|Array|SetArrayElem (Variables|Vars|GetEndRotationArray) _output_get (Variables|Vars|GetEndRotation)))))

(fn SetActiveDoorVars
  (bind _activedoorid (Variables|Vars|GetActiveDoorID))
  (Utilities|FlowControl|Sequence
    (:then_0
      (Variables|Vars|SetStartLocation (Utilities|Array|Get(acopy) (Variables|Vars|GetStartLocationArray) _activedoorid))
      (Variables|Vars|SetEndLocation (Utilities|Array|Get(acopy) (Variables|Vars|GetEndLocationArray) _activedoorid)))
    (:then_1
      (Variables|Vars|SetStartRotation (Utilities|Array|Get(acopy) (Variables|Vars|GetStartRotationArray) _activedoorid))
      (Variables|Vars|SetEndRotation (Utilities|Array|Get(acopy) (Variables|Vars|GetEndRotationArray) _activedoorid)))
    (:then_2
      (switch int (Variables|Vars|GetActiveDoorID)
        (:0
          (Variables|Vars|SetActiveDoor (Variables|Default|GetDoor_01_Inside)))
        (:1
          (Variables|Vars|SetActiveDoor (Variables|Default|GetDoor_02_MediumOutside)))
        (:2
          (Variables|Vars|SetActiveDoor (Variables|Default|GetDoor_03_Outside))))
      (return (Variables|Vars|GetActiveDoor)))))

(fn ResetVars
  (params (ID :type Integer))
  (bind _doorclose (Variables|Default|GetDoorClose))
  (bind _activedoorid (Variables|Vars|GetActiveDoorID))
  (LocalVariables|SetL_DoorID ID)
  (Utilities|FlowControl|Sequence
    (:then_0
      (LocalVariables|SetTempLocation (Variables|Vars|GetStartLocation))
      (bind _output_get (Variables|Vars|SetStartLocation (Variables|Vars|GetEndLocation)))
      (Utilities|Array|SetArrayElem (Variables|Vars|GetStartLocationArray) (LocalVariables|GetL_DoorID) _output_get)
      (bind _output_get_2 (Variables|Vars|SetEndLocation (LocalVariables|GetTempLocation)))
      (Utilities|Array|SetArrayElem (Variables|Vars|GetEndLocationArray) (LocalVariables|GetL_DoorID) _output_get_2))
    (:then_1
      (LocalVariables|SetTempRotation (Variables|Vars|GetStartRotation))
      (bind _output_get_3 (Variables|Vars|SetStartRotation (Variables|Vars|GetEndRotation)))
      (Utilities|Array|SetArrayElem (Variables|Vars|GetStartRotationArray) (LocalVariables|GetL_DoorID) _output_get_3)
      (bind _output_get_4 (Variables|Vars|SetEndRotation (LocalVariables|GetTempRotation)))
      (Utilities|Array|SetArrayElem (Variables|Vars|GetEndRotationArray) (LocalVariables|GetL_DoorID) _output_get_4))
    (:then_2
      (Utilities|Array|SetArrayElem _doorclose _activedoorid (not (Utilities|Array|Get(acopy) _doorclose _activedoorid)))
      (if (== (LocalVariables|GetL_DoorID) 2)
        (CallFunction|DoorMove 1)
        (elif (Variables|Default|GetInChain)
          (CallFunction|DoorMove (Variables|Vars|GetTempDoorID))
          (else
            (Variables|Default|SetIsMoving false)))))))

(fn Rotation
  (params (Moving :type Float%20%28single-precision%29))
  (Transformation|SetWorldLocation (Variables|Vars|GetActiveDoor) (Math|Vector|Lerp(Vector) (Variables|Vars|GetStartLocation) (Variables|Vars|GetEndLocation) Moving) false false)
  (Transformation|SetWorldRotation (Variables|Vars|GetActiveDoor) (Math|Rotator|Lerp(Rotator) (Variables|Vars|GetStartRotation) (Variables|Vars|GetEndRotation) Moving true) false false))

(fn СheckFunction
  (params (Selection :type Integer))
  (switch int Selection
    (:0
      (LocalVariables|SetL_tempID 2)
      (if (Utilities|Array|Get(acopy) (Variables|Default|GetDoorClose) (LocalVariables|GetL_tempID)) :!label _label
        (Variables|Default|SetInChain false)
        (else
          (Variables|Vars|SetTempDoorID (Variables|Vars|GetActiveDoorID))
          (Variables|Vars|SetActiveDoorID (LocalVariables|GetL_tempID))
          (Variables|Default|SetInChain true :!label _label_2))))
    (:1
      (if (Variables|Default|GetInChain)
        (Variables|Vars|SetTempDoorID 0)
        (goto _label_2)
        (else
          (Variables|Default|SetInChain false))))
    (:2
      (LocalVariables|SetL_tempID 0)
      (goto _label))))