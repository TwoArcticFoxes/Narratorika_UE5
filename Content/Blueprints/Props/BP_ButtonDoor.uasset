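; BP_ButtonDoor is an interactable button prop that, when available, relays a control call to its linked ControlActor, presumably a door.
; Interact and Control interface events share one path, which calls ControlInterface on that actor or CallDoorNotAvailable when unavailable.
; Outline events apply a green overlay material to the Cube on trace or for a timed scanner highlight, and clear it on close.
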(event EventBeginPlay
  (|CallParentFunction) ; This node is disabled and will not be called.\nDrag off pins to build functionality.
)

(event Collision|EventActorBeginOverlap
  (params (OtherActor :type Actor%20Object%20Reference))
  (|CallParentFunction OtherActor) ; This node is disabled and will not be called.\nDrag off pins to build functionality.
)

(event EventTick
  (params (DeltaSeconds :type Float%20%28single-precision%29))
  (|CallParentFunction DeltaSeconds) ; This node is disabled and will not be called.\nDrag off pins to build functionality.
)

(event EventOutlineInterface
  (params (Trace :type Boolean))
  ;[1 1 1] Outline
  (if Trace
    (Rendering|Material|SetOverlayMaterial (Variables|Default|GetCube) "/Game/Assets/Materials/My/MI_outlineGreen.MI_outlineGreen" :!class /Script/Engine.MeshComponent)
    (else
      (Rendering|Material|SetOverlayMaterial (Variables|Default|GetCube) 0 :!class /Script/Engine.MeshComponent))))

(event EventOutlineScannerOpen
  (params (Delay :type Float%20%28double-precision%29))
  ;[1 1 1] Outline
  (Rendering|Material|SetOverlayMaterial (Variables|Default|GetCube) "/Game/Assets/Materials/My/MI_outlineGreen.MI_outlineGreen" :!class /Script/Engine.MeshComponent)
  (Utilities|FlowControl|Delay Delay)
  (Rendering|Material|SetOverlayMaterial (Variables|Default|GetCube) 0 :!class /Script/Engine.MeshComponent))

(event EventOutlineClose
  ;[1 1 1] Outline
  (Rendering|Material|SetOverlayMaterial (Variables|Default|GetCube) 0 :!class /Script/Engine.MeshComponent))

(event EventInteractInterface
  ;[1 1 1] OpenDoor
  (if (Variables|Default|GetAvailable)
    (Default|ControlInterface (Variables|Default|GetControlActor))
    (else
      (Default|CallDoorNotAvailable))))

(event EventControlInterface
  ;[1 1 1] OpenDoor
  (if (Variables|Default|GetAvailable)
    (Default|ControlInterface (Variables|Default|GetControlActor))
    (else
      (Default|CallDoorNotAvailable))))

(fn ConstructionScript
  (|CallParentFunction))