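; Interactable electrical panel prop that the player repairs to restore electricity when the game instance reports it is off.
; Interacting shows a status widget bound to the panel and runs a looping timer that, on completion, sets HasElectricity and calls its dispatcher on BP_GameInstance.
; Trace and scanner events apply overlay outlines, green without power and red with it.
; A description component supplies the Russian name label.
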(event Custom|Repair
  ;[1 1 1] Interact Repair
  (Math|Float|IncrementFloat (Variables|Default|GetRepairProcess)
    (:%20%20
      (if (== (Variables|Default|GetRepairProcess) 6.0)
        (Utilities|Time|ClearandInvalidateTimerbyHandle (stale EventInteractInterface _returnvalue))
        (Development|SetHiddeninGame (Variables|Default|GetStatusWidget) true false)
        (bind _asbp_game_instance (Utilities|Casting|CastToBP_GameInstance (Game|GetGameInstance)))
        (bind _output_get (Variables|/Game/Blueprints/BP_GameInstance.BP_GameInstance_C|SetHasElectricity _asbp_game_instance true))
        (Default|CallHasElectricityDis _asbp_game_instance _output_get)))))

(event EventBeginPlay
  ;[1 1 1] BeginPlay
  (|CallParentFunction)
  (bind _aswb_electricity (Utilities|Casting|CastToWB_Electricity (UserInterface|GetUserWidgetObject (Variables|Default|GetStatusWidget))))
  (Variables|/Game/UI/BPWidgets/WB_Electricity.WB_Electricity_C|SetBP_Electricity _aswb_electricity self))

(event Collision|EventActorBeginOverlap
  (params (OtherActor :type Actor%20Object%20Reference))
  (|CallParentFunction OtherActor) ; This node is disabled and will not be called.\nDrag off pins to build functionality.
)

(event EventTick
  (params (DeltaSeconds :type Float%20%28single-precision%29))
  (|CallParentFunction DeltaSeconds) ; This node is disabled and will not be called.\nDrag off pins to build functionality.
)

(event EventInteractInterface
  ;[1 1 1] Interact Repair
  (bind _asbp_game_instance (Utilities|Casting|CastToBP_GameInstance (Game|GetGameInstance)))
  (if (not (Variables|/Game/Blueprints/BP_GameInstance.BP_GameInstance_C|GetHasElectricity _asbp_game_instance))
    (Development|SetHiddeninGame (Variables|Default|GetStatusWidget) false false)
    (bind _returnvalue (Utilities|Time|SetTimerbyEvent (delegate Custom|Repair) 1.0 true))))

(event EventOutlineClose
  ;[1 1 1] Outline
  (Rendering|Material|SetOverlayMaterial (Variables|Default|GetCube) 0 :!class /Script/Engine.MeshComponent)
  (Rendering|Material|SetOverlayMaterial (Variables|Default|GetCube1) 0 :!class /Script/Engine.MeshComponent)
  (Variables|Default|SetIsLight false))

(event EventObjectDescription
  (params (Trace :type Boolean))
  ;[1 1 1] Outline
  ;;[1 1 1] TextDescription
  (Default|Description (Variables|Default|GetBP_descriptionobject) Trace "Электрический щиток"))

(event EventOutlineScannerOpen
  (params (Delay :type Float%20%28double-precision%29))
  ;[1 1 1] Outline
  ;;[1 1 1] GameMode
  (if (not (Variables|Default|GetIsLight))
    (Variables|Default|SetIsLight true)
    (bind _asbp_game_instance (Utilities|Casting|CastToBP_GameInstance (Game|GetGameInstance)))
    (if (not (Variables|/Game/Blueprints/BP_GameInstance.BP_GameInstance_C|GetHasElectricity _asbp_game_instance))
      (Rendering|Material|SetOverlayMaterial (Variables|Default|GetCube) "/Game/Assets/Materials/My/MI_outlineGreen.MI_outlineGreen" :!class /Script/Engine.MeshComponent)
      (Rendering|Material|SetOverlayMaterial (Variables|Default|GetCube1) "/Game/Assets/Materials/My/MI_outlineGreen.MI_outlineGreen" :!class /Script/Engine.MeshComponent)
      (Utilities|FlowControl|Delay Delay)
      (Rendering|Material|SetOverlayMaterial (Variables|Default|GetCube) 0 :!class /Script/Engine.MeshComponent)
      (Rendering|Material|SetOverlayMaterial (Variables|Default|GetCube1) 0 :!class /Script/Engine.MeshComponent)
      (Variables|Default|SetIsLight false)
      (else
        (Rendering|Material|SetOverlayMaterial (Variables|Default|GetCube) "/Game/Assets/Materials/My/MI_outlineRed.MI_outlineRed" :!class /Script/Engine.MeshComponent)
        (Rendering|Material|SetOverlayMaterial (Variables|Default|GetCube1) "/Game/Assets/Materials/My/MI_outlineRed.MI_outlineRed" :!class /Script/Engine.MeshComponent)))))

(event EventOutlineInterface
  (params (Trace :type Boolean))
  ;[1 1 1] Outline
  ;;[1 1 1] Trace
  (if Trace
    (if (Variables|/Game/Blueprints/BP_GameInstance.BP_GameInstance_C|GetHasElectricity (.AsBP%20Game%20Instance (Utilities|Casting|CastToBP_GameInstance (Game|GetGameInstance))))
      (Rendering|Material|SetOverlayMaterial (Variables|Default|GetCube) "/Game/Assets/Materials/My/MI_outlineRed.MI_outlineRed" :!class /Script/Engine.MeshComponent)
      (Rendering|Material|SetOverlayMaterial (Variables|Default|GetCube1) "/Game/Assets/Materials/My/MI_outlineRed.MI_outlineRed" :!class /Script/Engine.MeshComponent)
      (else
        ;;;[1 1 1] Not
        (Rendering|Material|SetOverlayMaterial (Variables|Default|GetCube) "/Game/Assets/Materials/My/MI_outlineGreen.MI_outlineGreen" :!class /Script/Engine.MeshComponent)
        (Rendering|Material|SetOverlayMaterial (Variables|Default|GetCube1) "/Game/Assets/Materials/My/MI_outlineGreen.MI_outlineGreen" :!class /Script/Engine.MeshComponent)))
    (else
      (Rendering|Material|SetOverlayMaterial (Variables|Default|GetCube) 0 :!class /Script/Engine.MeshComponent)
      (Rendering|Material|SetOverlayMaterial (Variables|Default|GetCube1) 0 :!class /Script/Engine.MeshComponent))))

(fn ConstructionScript
  (|CallParentFunction))