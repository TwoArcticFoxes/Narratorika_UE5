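; Interactable workbench prop where the player becomes armored, advancing GameMode PlayerProgress from HaveArmor to Armored.
; Interaction works only at that stage, then fires PlayerArmored and sends a control interface message to the player character.
; Trace and scanner events overlay an outline on both lathe meshes, colored by progress: yellow before, green when usable, red after.
; A description object shows the Russian name and, when usable, the use prompt.
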(event EventBeginPlay
  (|CallParentFunction) ; This node is disabled and will not be called.\nDrag off pins to build functionality.
)

(event Collision|EventActorBeginOverlap
  (params (OtherActor :type Actor%20Object%20Reference))
  (|CallParentFunction OtherActor) ; This node is disabled and will not be called.\nDrag off pins to build functionality.
)

(event EventTick
  (params (DeltaSeconds :type Float%20%28single-precision%29))
  (|CallParentFunction DeltaSeconds) ; This node is disabled and will not be called.\nDrag off pins to build functionality.
)

(event EventOutlineClose
  ;[1 1 1] Outline
  (Rendering|Material|SetOverlayMaterial (Variables|Default|GetSM_Lathe1) 0 :!class /Script/Engine.MeshComponent)
  (Rendering|Material|SetOverlayMaterial (Variables|Default|GetSM_Lathe2) 0 :!class /Script/Engine.MeshComponent))

(event EventOutlineScannerOpen
  (params (Delay :type Float%20%28double-precision%29))
  ;[1 1 1] Outline
  (CallFunction|SetOutline)
  (Utilities|FlowControl|Delay Delay)
  (Rendering|Material|SetOverlayMaterial (Variables|Default|GetSM_Lathe1) 0 :!class /Script/Engine.MeshComponent)
  (Rendering|Material|SetOverlayMaterial (Variables|Default|GetSM_Lathe2) 0 :!class /Script/Engine.MeshComponent))

(event EventOutlineInterface
  (params (Trace :type Boolean))
  ;[1 1 1] Outline
  (if Trace
    (CallFunction|SetOutline)
    (else
      (Rendering|Material|SetOverlayMaterial (Variables|Default|GetSM_Lathe1) 0 :!class /Script/Engine.MeshComponent)
      (Rendering|Material|SetOverlayMaterial (Variables|Default|GetSM_Lathe2) 0 :!class /Script/Engine.MeshComponent))))

(event EventInteractInterface
  (bind _returnvalue (Game|GetGameMode))
  (bind _asbp_game_mode (Utilities|Casting|CastToBP_GameMode _returnvalue))
  ;[1 1 1] Interact
  (if (Utilities|Enum|Equal(Enum) "NewEnumerator2" (Variables|/Game/Blueprints/BP_GameMode.BP_GameMode_C|GetPlayerProgress _asbp_game_mode))
    (Variables|/Game/Blueprints/BP_GameMode.BP_GameMode_C|SetPlayerProgress _asbp_game_mode "NewEnumerator3")
    (Default|CallPlayerArmored)
    (Class|BPIInteractiveObject|ControlInterface(Message) (Game|GetPlayerCharacter 0))))

(event EventObjectActionDescription
  (params (Trace :type Boolean))
  ;[1 1 1] Description
  (if (Utilities|Enum|Equal(Enum) "NewEnumerator2" (Variables|/Game/Blueprints/BP_GameMode.BP_GameMode_C|GetPlayerProgress (.AsBP%20Game%20Mode (Utilities|Casting|CastToBP_GameMode (Game|GetGameMode)))))
    (Variables|Default|SetAction%20Descr%20Text_0 " <BoldH>[Е] Использовать </>")
    (else
      (Variables|Default|SetAction%20Descr%20Text_0 "")))
  (Default|ActionDescripton (Variables|Default|GetBP_descriptionobject) Trace (Variables|Default|GetAction%20Descr%20Text_0)))

(event EventObjectDescription
  (params (Trace :type Boolean))
  ;[1 1 1] Description
  (Default|Description (Variables|Default|GetBP_descriptionobject) Trace "Верстак"))

(fn ConstructionScript
  (|CallParentFunction))

(fn SetOutline
  (switch Utilities|FlowControl|Switch|SwitchonE_playerProgress (Variables|/Game/Blueprints/BP_GameMode.BP_GameMode_C|GetPlayerProgress (.AsBP%20Game%20Mode (Utilities|Casting|CastToBP_GameMode (Game|GetGameMode))))
    (:NewEnumerator5
      (Rendering|Material|SetOverlayMaterial (Variables|Default|GetSM_Lathe1) "/Game/Assets/Materials/My/MI_outlineYe.MI_outlineYe" :!class /Script/Engine.MeshComponent :!label _label)
      (Rendering|Material|SetOverlayMaterial (Variables|Default|GetSM_Lathe2) "/Game/Assets/Materials/My/MI_outlineYe.MI_outlineYe" :!class /Script/Engine.MeshComponent))
    (:NewEnumerator4
      (goto _label))
    (:NewEnumerator0
      (goto _label))
    (:NewEnumerator1
      (goto _label))
    (:NewEnumerator2
      (Rendering|Material|SetOverlayMaterial (Variables|Default|GetSM_Lathe1) "/Game/Assets/Materials/My/MI_outlineGreen.MI_outlineGreen" :!class /Script/Engine.MeshComponent)
      (Rendering|Material|SetOverlayMaterial (Variables|Default|GetSM_Lathe2) "/Game/Assets/Materials/My/MI_outlineGreen.MI_outlineGreen" :!class /Script/Engine.MeshComponent))
    (:NewEnumerator3
      (Rendering|Material|SetOverlayMaterial (Variables|Default|GetSM_Lathe1) "/Game/Assets/Materials/My/MI_outlineRed.MI_outlineRed" :!class /Script/Engine.MeshComponent)
      (Rendering|Material|SetOverlayMaterial (Variables|Default|GetSM_Lathe2) "/Game/Assets/Materials/My/MI_outlineRed.MI_outlineRed" :!class /Script/Engine.MeshComponent))))