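; BP_descriptionobject relays object description and action description text to the player's HUD widget.
; On BeginPlay it waits briefly, then casts the first player's HUD to BP_HUD_Diploma and caches its UMG widget reference.
; Its two events forward their text to the matching widget events when the trace flag is true and send an empty string otherwise, clearing the prompt.
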(event Custom|description
  (params (Trace :type Boolean) (Text :type Text))
  (bind _umg_hud_ref (Variables|Default|GetUMG%20HUD%20Ref))
  (if Trace
    (Default|EventDescription _umg_hud_ref Text)
    (else
      (Default|EventDescription _umg_hud_ref " "))))

(event Custom|ActionDescripton
  (params (Trace :type Boolean) (ActionDescrText :type Text))
  (bind _umg_hud_ref (Variables|Default|GetUMG%20HUD%20Ref))
  (if Trace
    (Default|EventActionDescription _umg_hud_ref ActionDescrText)
    (else
      (Default|EventActionDescription _umg_hud_ref " "))))

(event EventBeginPlay
  (Utilities|FlowControl|Delay 0.2)
  (bind _asbp_hud_diploma (Utilities|Casting|CastToBP_HUD_Diploma (HUD|GetHUD (Game|GetPlayerController 0))))
  (Variables|Default|SetUMG%20HUD%20Ref (Variables|/Game/Blueprints/BP_HUD_Diploma.BP_HUD_Diploma_C|GetUMG_HUD_ref _asbp_hud_diploma)))