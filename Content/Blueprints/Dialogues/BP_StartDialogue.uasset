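; Interactable actor that plays the game's opening UI sequence, ending in the start dialogue.
; On interact it shows UMG_StartGameInst, whose completion event leads after short delays to the death screen and then UMG_dialogue fed by DT_StartDialogue.
; Each stage switches input to UI-only.
; The dialogue's camera-possess event removes the dialogue and death screen, restores game input and fires the PossessCameraDialogue dispatcher.
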(event Custom|PossessCamera
  (bind _returnvalue (Game|GetPlayerController 0))
  ;[1 1 1] Create Widget Dialogue
  ;;[1 1 1] Delete
  (Utilities|FlowControl|Sequence
    (:then_0
      (Widget|RemovefromParent (stale Custom|CreateWidgetDialogueEvent _returnvalue_2))
      (Widget|RemovefromParent (Variables|Default|GetDeathScreenW))
      (Input|SetInputModeGameOnly _returnvalue false)
      (Variables|/Script/Engine.PlayerController|SetbShowMouseCursor _returnvalue false))
    (:then_1
      (Default|CallPossessCameraDialogue))))

(event Custom|CreateWidgetDialogueEvent
  (bind _returnvalue (Game|GetPlayerController 0))
  ;[1 1 1] Create Widget Dialogue
  ;;[1 1 1] Create
  (bind _returnvalue_2 (UserInterface|CreateWidget "/Game/UI/UMG_dialogue.UMG_dialogue_C" _returnvalue "/Game/Blueprints/Dialogues/DT_StartDialogue.DT_StartDialogue"))
  (EventDispatchers|BindEventtoPossesCamera _returnvalue_2 (delegate Custom|PossessCamera))
  (UserInterface|Viewport|AddtoViewport _returnvalue_2 0)
  (Input|SetInputModeUIOnly _returnvalue 0 "DoNotLock" false)
  (Variables|/Script/Engine.PlayerController|SetbShowMouseCursor _returnvalue true))

(event Custom|DeathScreenWidget
  (bind _returnvalue (Game|GetPlayerController 0))
  ;[1 1 1] DeathScreen Event
  (bind _returnvalue_2 (UserInterface|CreateWidget "/Game/UI/Start/UMG_DeathScreen.UMG_DeathScreen_C" _returnvalue))
  (UserInterface|Viewport|AddtoViewport _returnvalue_2 0)
  (Variables|Default|SetDeathScreenW _returnvalue_2)
  (Input|SetInputModeUIOnly _returnvalue 0 "DoNotLock" false)
  (Utilities|FlowControl|Delay 9.0)
  (CallFunction|CreateWidgetDialogueEvent))

(event Custom|StartInst
  (bind _returnvalue (Game|GetPlayerController 0))
  ;[1 1 1] StartInst
  (bind _returnvalue_2 (UserInterface|CreateWidget "/Game/UI/Start/UMG_StartGameInst.UMG_StartGameInst_C" _returnvalue))
  (UserInterface|Viewport|AddtoViewport _returnvalue_2 0)
  (EventDispatchers|BindEventtoPresentationDone _returnvalue_2 (delegate Custom|Done))
  (Input|SetInputModeUIOnly _returnvalue 0 "DoNotLock" false))

(event Custom|Done
  (params (Done :type Boolean))
  ;[1 1 1] StartInst
  (Utilities|FlowControl|Delay 1.0)
  (CallFunction|DeathScreenWidget)
  (Widget|RemovefromParent (stale Custom|StartInst _returnvalue_2)))

(event EventInteractInterface
  (CallFunction|StartInst))

(event Collision|EventActorBeginOverlap
  (params (OtherActor :type Actor%20Object%20Reference))
  (|CallParentFunction OtherActor) ; This node is disabled and will not be called.\nDrag off pins to build functionality.
)

(event EventTick
  (params (DeltaSeconds :type Float%20%28single-precision%29))
  (|CallParentFunction DeltaSeconds) ; This node is disabled and will not be called.\nDrag off pins to build functionality.
)

(event EventBeginPlay
  (|CallParentFunction) ; This node is disabled and will not be called.\nDrag off pins to build functionality.
)

(fn ConstructionScript
  (|CallParentFunction))