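; BP_NPCDialogue plays an NPC dialogue by showing DataTable rows in sequence as hint messages on the UMG HUD.
; StartDialogue records the HUD's current array index, creates the row's hint, then re-calls itself after a fixed delay until rows run out.
; A looping timer, started after a delay scaled by row count, calls ENDRepl to end hints by an incrementing counter and clears itself upon reaching the row count.
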(event Custom|StartDialogue
  ;[1 1 1] Dialogue
  ;;[1 1 1] Rows
  (bind _outrownames (DataTable|GetDataTableRowNames (Variables|Default|GetDialogueTable)))
  (Variables|Default|SetMaxRowID (Utilities|Array|Length _outrownames))
  (Variables|Default|SetCurrentRowName (Utilities|Array|Get(acopy) _outrownames (Variables|Default|GetCurrentRow)))
  ;;[1 1 1] get HUD
  (bind _asbp_hud_diploma (Utilities|Casting|CastToBP_HUD_Diploma (HUD|GetHUD (Game|GetPlayerController 0))))
  (bind _output_get (Variables|Default|SetUMG%20HUD%20Ref (Variables|/Game/Blueprints/BP_HUD_Diploma.BP_HUD_Diploma_C|GetUMG_HUD_ref _asbp_hud_diploma)))
  ;;;[1 1 1] Repl Array
  (bind _output_get_2 (Variables|Default|SetArray%20Index%20HUD (Variables|/Game/UI/UMG_HUD.UMG_HUD_C|GetArrayIndex _output_get)))
  (Utilities|Array|SetArrayElem (Variables|Default|GetIndexArray) (Variables|Default|GetIndex) _output_get_2 true)
  (Math|Integer|IncrementInt (Variables|Default|GetIndex)
    (:%20%20
      (Class|BPIHints|CreateHint(Message) (Variables|Default|GetUMG%20HUD%20Ref) (Variables|Default|GetDialogueTable) (Variables|Default|GetCurrentRowName))
      ;;[1 1 1] NextRepl
      (Math|Integer|IncrementInt (Variables|Default|GetCurrentRow)
        (:%20%20
          (if (< (Variables|Default|GetCurrentRow) (Variables|Default|GetMaxRowID))
            (Utilities|FlowControl|Delay 3.0)
            (CallFunction|StartDialogue)
            ;[1 1 1] Timer for End
            (if (not (Utilities|Time|IsValidTimerHandle (Variables|Default|GetTimer)))
              (Utilities|FlowControl|Delay (* (Variables|Default|GetMaxRowID) (Variables|Default|GetTime)))
              ;;[1 1 1] Timer
              (bind _returnvalue (Utilities|Time|SetTimerbyEvent (delegate Custom|END%20repl) (Variables|Default|GetTime) true))
              (Variables|Default|SetTimer _returnvalue))))))))

(event Custom|END%20repl
  ;[1 1 1] Timer for End
  ;;[1 1 1] Timer
  ;;;[1 1 1] ClearRepl
  (Default|EndHint (Variables|Default|GetUMG%20HUD%20Ref) (Variables|Default|GetEndIndex))
  (Math|Integer|IncrementInt (Variables|Default|GetEndIndex)
    (:%20%20
      (if (== (+ (Variables|Default|GetCurrentRow) 1) (Variables|Default|GetEndIndex))
        (Utilities|Time|ClearandInvalidateTimerbyHandle (Variables|Default|GetTimer))))))

(fn ConstructionScript)