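; BP_InteractiveNPC is an NPC that opens a dialogue UI when its Interact event fires.
; Interact clears all widgets, shows UMG_DialogeTestGround, and switches player 0 to UI-only input with a visible cursor.
; It binds EndWidget to the dialogue's button-click callback.
; EndWidget removes the dialogue, creates a fresh UMG_HUD_testground, and restores game-only input with the cursor hidden.
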(event Custom|EndWidget
  (bind _returnvalue (Game|GetPlayerController 0))
  (Widget|RemovefromParent (stale EventInteract _returnvalue_2))
  (bind _returnvalue_2 (UserInterface|CreateWidget "/Game/UI/Homework/UMG_HUD_testground.UMG_HUD_testground_C"))
  (UserInterface|Viewport|AddtoViewport _returnvalue_2 0)
  (Input|SetInputModeGameOnly _returnvalue false)
  (Variables|/Script/Engine.PlayerController|SetbShowMouseCursor _returnvalue false))

(event EventInteract
  (bind _returnvalue (Game|GetPlayerController 0))
  (Viewport|RemoveAllWidgets)
  (bind _returnvalue_2 (UserInterface|CreateWidget "/Game/UI/Homework/UMG_DialogeTestGround.UMG_DialogeTestGround_C"))
  (EventDispatchers|BindEventtoDialogeClickonButton _returnvalue_2 (delegate Custom|EndWidget))
  (UserInterface|Viewport|AddtoViewport _returnvalue_2 0)
  (Input|SetInputModeUIOnly _returnvalue 0 "DoNotLock" false)
  (Variables|/Script/Engine.PlayerController|SetbShowMouseCursor _returnvalue true))

(fn ConstructionScript
  (|CallParentFunction))