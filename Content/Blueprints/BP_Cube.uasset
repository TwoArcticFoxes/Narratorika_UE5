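; BP_Cube is a cube actor that shuttles back and forth between its start location and an offset end point, reporting what it touches.
; BeginPlay turns EndLocation into a world position, then a timeline lerps the location without sweep, swapping endpoints and replaying on each finish.
; Timeline speed comes from PlayRateTimeline divided by PlayRateTimelineMod.
; Hit and overlap events print whether the other actor is BP_Cube, BP_ThirdPersonCharacter, BP_sphere or something else.
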(event OnComponentHit(Cube)
  (params (HitComponent :type Primitive%20Component%20Object%20Reference) (OtherActor :type Actor%20Object%20Reference) (OtherComp :type Primitive%20Component%20Object%20Reference) (NormalImpulse :type Vector :default "0, 0, 0") (Hit :type Hit%20Result%20Structure%20%28by%20ref%29))
  ;[1 1 1] Hit
  (Utilities|Casting|CastToBP_Cube OtherActor
    (:then
      (Development|PrintString "Hit BP_Cube" true true "(R=0.000000,G=0.660000,B=1.000000,A=1.000000)" 1e+01))
    (:CastFailed
      (Utilities|Casting|CastToBP_ThirdPersonCharacter OtherActor
        (:then
          (Development|PrintString "Hit PersonChatracter" true true "(R=0.000000,G=1.000000,B=0.034738,A=1.000000)"))
        (:CastFailed
          (Utilities|Casting|CastToBP_sphere OtherActor
            (:then
              (Development|PrintString "Hit BP_sphere" true true "(R=1.000000,G=0.927710,B=0.000000,A=1.000000)"))
            (:CastFailed
              (Development|PrintString "Hit Other" true true "(R=1.000000,G=0.000000,B=0.001717,A=1.000000)"))))))))

(event OnComponentBeginOverlap(Cube)
  (params (OverlappedComponent :type Primitive%20Component%20Object%20Reference) (OtherActor :type Actor%20Object%20Reference) (OtherComp :type Primitive%20Component%20Object%20Reference) (OtherBodyIndex :type Integer) (bFromSweep :type Boolean) (SweepResult :type Hit%20Result%20Structure%20%28by%20ref%29))
  ;[1 1 1] Overlap
  (Utilities|Casting|CastToBP_Cube OtherActor
    (:then
      (Development|PrintString "Overlap BP_Cube" true true "(R=0.000000,G=0.660000,B=1.000000,A=1.000000)" 1e+01))
    (:CastFailed
      (Utilities|Casting|CastToBP_ThirdPersonCharacter OtherActor
        (:then
          (Development|PrintString "Overlap PersonChatracter" true true "(R=0.000000,G=1.000000,B=0.034738,A=1.000000)"))
        (:CastFailed
          (Utilities|Casting|CastToBP_sphere OtherActor
            (:then
              (Development|PrintString "Overlap BP_sphere" true true "(R=1.000000,G=0.927710,B=0.000000,A=1.000000)"))
            (:CastFailed
              (Development|PrintString "Overlap Other" true true "(R=1.000000,G=0.000000,B=0.001717,A=1.000000)"))))))))

(event Custom|StartMoving
  ;[1 1 1] StartMoving Timeline
  (Components|Timeline|SetPlayRate (Variables|Default|GetMoving%20Timeline) (/ (Variables|Default|GetPlayRateTimeline) (Variables|Default|GetPlayRateTimelineMod)))
  (bind _moving (Timeline|Moving%20Timeline PlayFromStart)
    (:Update
      (Transformation|SetActorLocation (Math|Vector|Lerp(Vector) (Variables|Default|GetStartLocation) (Variables|Default|GetEndLocation) _moving) false false))
    (:Finished
      (Variables|Default|SetTempLocation (Variables|Default|GetStartLocation))
      (Variables|Default|SetStartLocation (Variables|Default|GetEndLocation))
      (Variables|Default|SetEndLocation (Variables|Default|GetTempLocation))
      (CallFunction|StartMoving))))

(event EventBeginPlay
  ;[1 1 1] Begin play
  (bind _output_get (Variables|Default|SetStartLocation (Transformation|GetActorLocation)))
  (Variables|Default|SetEndLocation (+ _output_get (Variables|Default|GetEndLocation)))
  (CallFunction|StartMoving))

(event Collision|EventActorBeginOverlap
  (params (OtherActor :type Actor%20Object%20Reference)))

(event EventTick
  (params (DeltaSeconds :type Float%20%28single-precision%29)))

(fn ConstructionScript)