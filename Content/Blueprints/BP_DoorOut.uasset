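; Door actor that slides and rotates between its placed transform and a relative end offset when triggered through a control interface.
; If it can open, it waits a delay and runs a rate-adjusted timeline lerp; otherwise it fires NeedBeOpen, leaving its moved guard set.
; On finish, repeatable doors swap endpoints and re-arm, and a FlipFlop alternates the Close state broadcast through Hodor.
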(event Custom|StartMoving
  ;[1 1 1] StartMoving Timeline
  (CallFunction|PlayRateFunction)
  (bind _moving (Timeline|MovingTimeline PlayFromStart)
    (:Update
      (Transformation|SetActorLocation (Math|Vector|Lerp(Vector) (Variables|Place|GetStartLocation) (Variables|Place|GetEndLocation) _moving) false false)
      (Transformation|SetActorRotation (Math|Rotator|Lerp(Rotator) (Variables|Place|GetStartRotator) (Variables|Place|GetEndRotator) _moving)))
    (:Finished
      (CallFunction|ResetVars)
      (Utilities|FlowControl|FlipFlop
        (:A
          (Variables|CanbeOpen|SetClose false))
        (:B
          (Variables|CanbeOpen|SetClose true)))
      (Default|CallHodor (Variables|CanbeOpen|GetClose)))))

(event EventBeginPlay
  ;[1 1 1] BeginPlay
  (|CallParentFunction)
  (CallFunction|SetVars))

(event EventControlInterface
  ;[1 1 1] Control
  (if (not (Variables|Control|GetIsMoved))
    (Variables|Control|SetIsMoved true)
    (if (Variables|CanBeOpen|GetCanBeOpen)
      (Utilities|FlowControl|Delay (Variables|Control|GetDelay))
      (CallFunction|StartMoving)
      (else
        (Default|CallNeedbeOpen)))))

(fn ConstructionScript
  (|CallParentFunction))

(fn PlayRateFunction
  (Components|Timeline|SetPlayRate (Variables|Default|GetMovingTimeline) (/ (Variables|MovingTimeline|GetPlayRate) (Variables|MovingTimeline|GetPlayRateMod))))

(fn SetVars
  (bind _output_get (Variables|Place|SetStartLocation (Transformation|GetActorLocation)))
  (Variables|Place|SetEndLocation (+ _output_get (Variables|Place|GetEndLocation)))
  (bind _output_get_2 (Variables|Place|SetStartRotator (Transformation|GetActorRotation)))
  (Variables|Place|SetEndRotator (Math|Rotator|CombineRotators _output_get_2 (Variables|Place|GetEndRotator))))

(fn ResetVars
  (if (Variables|MovingTimeline|GetIsRepeat)
    (Variables|Place|SetTempLocation (Variables|Place|GetStartLocation))
    (Variables|Place|SetStartLocation (Variables|Place|GetEndLocation))
    (Variables|Place|SetEndLocation (Variables|Place|GetTempLocation))
    (Variables|Place|SetTempRotator (Variables|Place|GetStartRotator))
    (Variables|Place|SetStartRotator (Variables|Place|GetEndRotator))
    (Variables|Place|SetEndRotator (Variables|Place|GetTempRotator))
    (Variables|Control|SetIsMoved false)))