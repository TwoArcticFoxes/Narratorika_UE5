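; Procedural server prop that builds a vertical stack of up to eleven randomly chosen static mesh modules in its Construction Script.
; The Random flag rerolls module types and gaps, then clears itself so the stored layout persists across rebuilds.
; LocationFunc places the lower five unconditionally, each returning the next Z offset.
; LocationFunc2 and the final switch place upper modules, mostly gated by per-type height limits.
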(event EventBeginPlay)

(event Collision|EventActorBeginOverlap
  (params (OtherActor :type Actor%20Object%20Reference)))

(event EventTick
  (params (DeltaSeconds :type Float%20%28single-precision%29)))

(fn ConstructionScript
  (bind _returnvalue (Math|Random|RandomInteger 6))
  (bind _returnvalue_2 (Math|Random|RandomFloatinRange -1.0 5.0))
  (if (Variables|Settings|GetRandom)
    (Variables|Settings|SetModule%201%20 _returnvalue)
    (Variables|Settings|SetModule%202 _returnvalue)
    (Variables|Settings|SetModule%203 _returnvalue)
    (Variables|Settings|SetModule%204 _returnvalue)
    (Variables|Settings|SetModule%205 _returnvalue)
    (Variables|Settings|SetModule%206 _returnvalue)
    (Variables|Settings|SetModule%207 _returnvalue)
    (Variables|Settings|SetModule%208 _returnvalue)
    (Variables|Settings|SetModule%209 _returnvalue)
    (Variables|Settings|SetModule%2010 _returnvalue)
    (Variables|Settings|SetModule%2011 _returnvalue)
    (Variables|Settings|SetRandom%20Int%2001 _returnvalue_2)
    (Variables|Settings|SetRandom%20Int%2002 _returnvalue_2)
    (Variables|Settings|SetRandom%20Int%2003 _returnvalue_2)
    (Variables|Settings|SetRandom%20Int%2004 _returnvalue_2)
    (Variables|Settings|SetRandom%20Int%2005 _returnvalue_2)
    (Variables|Settings|SetRandom%20Int%2006 _returnvalue_2)
    (Variables|Settings|SetRandom%20Int%2007 _returnvalue_2)
    (Variables|Settings|SetRandom%20Int%2008 _returnvalue_2)
    (Variables|Settings|SetRandom%20Int%2009 _returnvalue_2)
    (Variables|Settings|SetRandom%20Int%2010 _returnvalue_2)
    (Variables|Settings|SetRandom false))
  ;[1 1 1] MODULE 01-05
  (CallFunction|LocationFunc (Variables|Settings|GetRandom%20Int%2001) (Variables|Settings|GetModule%201%20) "0, 0, 0")
  (bind _output_get (Variables|Settings|SetLocation%201 (Variables|Default|GetLocation)))
  (CallFunction|LocationFunc (Variables|Settings|GetRandom%20Int%2002) (Variables|Settings|GetModule%202) _output_get)
  (bind _output_get_2 (Variables|Settings|SetLocation%202 (Variables|Default|GetLocation)))
  (CallFunction|LocationFunc (Variables|Settings|GetRandom%20Int%2003) (Variables|Settings|GetModule%203) _output_get_2)
  (bind _output_get_3 (Variables|Settings|SetLocation%203 (Variables|Default|GetLocation)))
  (CallFunction|LocationFunc (Variables|Settings|GetRandom%20Int%2004) (Variables|Settings|GetModule%204) _output_get_3)
  (bind _output_get_4 (Variables|Settings|SetLocation%204 (Variables|Default|GetLocation)))
  (CallFunction|LocationFunc (Variables|Settings|GetRandom%20Int%2005) (Variables|Settings|GetModule%205) _output_get_4)
  (bind _output_get_5 (Variables|Settings|SetLocation%205 (Variables|Default|GetLocation)))
  ;[1 1 1] MODULE 06-10
  (CallFunction|LocationFunc2 (Variables|Settings|GetRandom%20Int%2006) (Variables|Settings|GetModule%206) _output_get_5)
  (bind _output_get_6 (Variables|Settings|SetLocation%206 (Variables|Default|GetLocation)))
  (CallFunction|LocationFunc2 (Variables|Settings|GetRandom%20Int%2007) (Variables|Settings|GetModule%207) _output_get_6)
  (bind _output_get_7 (Variables|Settings|SetLocation%207 (Variables|Default|GetLocation)))
  (CallFunction|LocationFunc2 (Variables|Settings|GetRandom%20Int%2008) (Variables|Settings|GetModule%208) _output_get_7)
  (bind _output_get_8 (Variables|Settings|SetLocation%208 (Variables|Default|GetLocation)))
  (CallFunction|LocationFunc2 (Variables|Settings|GetRandom%20Int%2009) (Variables|Settings|GetModule%209) _output_get_8)
  (bind _output_get_9 (Variables|Settings|SetLocation%209 (Variables|Default|GetLocation)))
  (CallFunction|LocationFunc2 (Variables|Settings|GetRandom%20Int%2010) (Variables|Settings|GetModule%2010) _output_get_9)
  (Variables|Settings|SetLocation%2010 (Variables|Default|GetLocation))
  ;[1 1 1] MODULE 11
  (switch int (Variables|Settings|GetModule%2011)
    (:Default
      (Math|Float|CompareFloat (.Z (Math|Vector|BreakVector (Variables|Settings|GetLocation%2010))) 198.0 :!label _label
        (:<
          (AddComponent|AddStaticMeshComponent false (Math|Conversions|ToTransform(Vector) (Variables|Settings|GetLocation%2010))))))
    (:0
      (goto _label))
    (:1
      (Math|Float|CompareFloat (.Z (Math|Vector|BreakVector (Variables|Settings|GetLocation%2010))) 194.0
        (:<
          (AddComponent|AddStaticMeshComponent false (Math|Conversions|ToTransform(Vector) (Variables|Settings|GetLocation%2010))))))
    (:2
      (Math|Float|CompareFloat (.Z (Math|Vector|BreakVector (Variables|Settings|GetLocation%2010))) 184.0
        (:<
          (AddComponent|AddStaticMeshComponent false (Math|Conversions|ToTransform(Vector) (Variables|Settings|GetLocation%2010))))))
    (:3
      (Math|Float|CompareFloat (.Z (Math|Vector|BreakVector (Variables|Settings|GetLocation%2010))) 188.0
        (:<
          (AddComponent|AddStaticMeshComponent false (Math|Conversions|ToTransform(Vector) (Variables|Settings|GetLocation%2010))))))
    (:4
      (Math|Float|CompareFloat (.Z (Math|Vector|BreakVector (Variables|Settings|GetLocation%2010))) 176.0
        (:<
          (AddComponent|AddStaticMeshComponent false (Math|Conversions|ToTransform(Vector) (Variables|Settings|GetLocation%2010))))))
    (:5
      (Math|Float|CompareFloat (.Z (Math|Vector|BreakVector (Variables|Settings|GetLocation%2010))) 184.0
        (:<
          (AddComponent|AddStaticMeshComponent false (Math|Conversions|ToTransform(Vector) (Variables|Settings|GetLocation%2010))))))))

(fn LocationFunc
  (params (InputPin :type Float%20%28double-precision%29) (Selection :type Integer) (InLocation :type Vector))
  (bind _returnvalue (Math|Conversions|ToTransform(Vector) InLocation))
  (bind _z (Math|Vector|BreakVector InLocation))
  (bind _returnvalue_2 (+ InputPin _z))
  (bind _returnvalue_3 (Math|Vector|MakeVector 0.0 0.0 _returnvalue_2))
  (switch int Selection
    (:Default
      (AddComponent|AddStaticMeshComponent false _returnvalue :!label _label)
      (Variables|Default|SetLocation (+ _returnvalue_3 "0, 0,20.000000")))
    (:0
      (goto _label))
    (:1
      (AddComponent|AddStaticMeshComponent false _returnvalue)
      (Variables|Default|SetLocation (+ _returnvalue_3 "0, 0,24.000000")))
    (:2
      (AddComponent|AddStaticMeshComponent false _returnvalue)
      (Variables|Default|SetLocation (+ _returnvalue_3 "0, 0,36.000000")))
    (:3
      (AddComponent|AddStaticMeshComponent false _returnvalue)
      (Variables|Default|SetLocation (+ _returnvalue_3 "0, 0,30.000000")))
    (:4
      (AddComponent|AddStaticMeshComponent false _returnvalue)
      (Variables|Default|SetLocation (+ _returnvalue_3 "0, 0,44.000000")))
    (:5
      (AddComponent|AddStaticMeshComponent false _returnvalue)
      (Variables|Default|SetLocation (+ _returnvalue_3 "0, 0,36.000000")))))

(fn LocationFunc2
  (params (InputPin :type Float%20%28double-precision%29) (Selection :type Integer) (InLocation :type Vector))
  (bind _z (Math|Vector|BreakVector InLocation))
  (bind _returnvalue (Math|Conversions|ToTransform(Vector) InLocation))
  (bind _z_2 (Math|Vector|BreakVector InLocation))
  (bind _returnvalue_2 (+ InputPin _z_2))
  (bind _returnvalue_3 (Math|Vector|MakeVector 0.0 0.0 _returnvalue_2))
  (switch int Selection
    (:Default
      (Math|Float|CompareFloat _z 198.0 :!label _label
        (:<
          (AddComponent|AddStaticMeshComponent false _returnvalue)
          (Variables|Default|SetLocation (+ _returnvalue_3 "0, 0,20.000000")))))
    (:0
      (goto _label))
    (:1
      (Math|Float|CompareFloat _z 194.0
        (:<
          (AddComponent|AddStaticMeshComponent false _returnvalue)
          (Variables|Default|SetLocation (+ _returnvalue_3 "0, 0,24.000000")))))
    (:2
      (Math|Float|CompareFloat _z 184.0
        (:<
          (AddComponent|AddStaticMeshComponent false _returnvalue)
          (Variables|Default|SetLocation (+ _returnvalue_3 "0, 0,36.000000")))))
    (:3
      (Math|Float|CompareFloat _z 188.0))
    (:4
      (Math|Float|CompareFloat _z 176.0
        (:>
          (AddComponent|AddStaticMeshComponent false _returnvalue)
          (Variables|Default|SetLocation (+ _returnvalue_3 "0, 0,44.000000")))
        (:<
          (AddComponent|AddStaticMeshComponent false _returnvalue)
          (Variables|Default|SetLocation (+ _returnvalue_3 "0, 0,30.000000")))))
    (:5
      (Math|Float|CompareFloat _z 184.0
        (:<
          (AddComponent|AddStaticMeshComponent false _returnvalue)
          (Variables|Default|SetLocation (+ _returnvalue_3 "0, 0,36.000000")))))))