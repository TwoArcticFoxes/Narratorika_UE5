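; Charging station prop for cleaner actors, which sends them charging messages once it has electricity.
; It binds to the game instance's electricity event, which shows the ON component, hides OFF and messages the stored cleaner.
; Box overlaps send start and stop charging messages when powered; without power, an entering BPI_Cleaner actor is stored until an overlap ends.
; The construction script sets the initial ON/OFF visibility from HasElectricity.
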(event OnComponentBeginOverlap(Box)
  (params (OverlappedComponent :type Primitive%20Component%20Object%20Reference) (OtherActor :type Actor%20Object%20Reference) (OtherComp :type Primitive%20Component%20Object%20Reference) (OtherBodyIndex :type Integer) (bFromSweep :type Boolean) (SweepResult :type Hit%20Result%20Structure%20%28by%20ref%29))
  (if (Variables|Default|GetHasElectricity)
    (Class|BPICleaner|ChargingCleaner(Message) OtherActor)
    (elif (Utilities|DoesObjectImplementInterface OtherActor "/Game/Blueprints/BPI/BPI_Cleaner.BPI_Cleaner_C")
      (Variables|Default|SetCleaner OtherActor))))

(event OnComponentEndOverlap(Box)
  (params (OverlappedComponent :type Primitive%20Component%20Object%20Reference) (OtherActor :type Actor%20Object%20Reference) (OtherComp :type Primitive%20Component%20Object%20Reference) (OtherBodyIndex :type Integer))
  (if (Variables|Default|GetHasElectricity)
    (Class|BPICleaner|StopCharging(Message) OtherActor))
  (Utilities|IsValid (Variables|Default|GetCleaner)
    (:Is%20Valid
      (Variables|Default|SetCleaner 0))))

(event Custom|CustomEvent
  (params (HasElectricity :type Boolean))
  ;[1 1 1] Has Electricity
  (Variables|Default|SetHasElectricity HasElectricity)
  (Development|SetHiddeninGame (Variables|Default|GetOFF) true false)
  (Development|SetHiddeninGame (Variables|Default|GetON) false false)
  (Class|BPICleaner|ChargingCleaner(Message) (Variables|Default|GetCleaner)))

(event EventBeginPlay
  ;[1 1 1] Has Electricity
  (|CallParentFunction)
  (bind _asbp_game_instance (Utilities|Casting|CastToBP_GameInstance (Game|GetGameInstance)))
  (EventDispatchers|BindEventtoHasElectricityDis _asbp_game_instance (delegate Custom|CustomEvent)))

(event Collision|EventActorBeginOverlap
  (params (OtherActor :type Actor%20Object%20Reference))
  (|CallParentFunction OtherActor) ; This node is disabled and will not be called.\nDrag off pins to build functionality.
)

(event EventTick
  (params (DeltaSeconds :type Float%20%28single-precision%29))
  (|CallParentFunction DeltaSeconds) ; This node is disabled and will not be called.\nDrag off pins to build functionality.
)

(fn ConstructionScript
  (|CallParentFunction)
  (if (Variables|Default|GetHasElectricity)
    (Development|SetHiddeninGame (Variables|Default|GetOFF) true false)
    (else
      (Development|SetHiddeninGame (Variables|Default|GetON) true false))))